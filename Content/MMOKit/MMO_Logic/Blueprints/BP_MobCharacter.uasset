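; Base mob character for the MMO kit, configured from StartingStats with nameplate, loot and respawn.
; On non-cosmetic (server) BeginPlay it adds stats and AI components and grants a default attack.
; An event bus relays target changes, which toggle walk/run speed, and aggro-range events for hostile mobs.
; On death it awards XP to the killer, rolls a loot bag, asks GameMode for a delayed respawn, then destroys itself.
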(event `self.SetNameplateWidget`
  ;[1 0.312 0.302] Set NamePlate Widget (called from BaseCharacter on BeginPlay)
  (bind _returnvalue (`|CreateWidget` "/Game/MMOKit/MMO_Logic/Widgets/WBP_MobNameplate.WBP_MobNameplate_C" null self))
  (`WidgetComponent.SetWidget` (`self.NameplateWidget`) _returnvalue))

(event `self.ReceiveBeginPlay`
  (bind _statscomp (`self.StatsComp`))
  (bind (_mobname _hp) (break `/Game/MMOKit/MMO_Logic/Blueprints/Struct/FStatsMob` (`self.StartingStats`)))
  (bind ((`WalkSpeed_27_B4ED4B7F4467BA5F8EDA16BA418DB696` _walkspeed) (`RunSpeed_26_7DDAD1874B5FF67DE51250A5E27EC5B2` _runspeed)) (break `/Game/MMOKit/MMO_Logic/Blueprints/Struct/FStatsMob` (`self.StartingStats`)))
  (set `self.MaxMoveSpeed` _runspeed)
  (`parent.ReceiveBeginPlay`)
  (set `CharacterMovementComponent.MaxWalkSpeed` _walkspeed (`self.CharacterMovement`))
  (`MmoUtilities.LogString` "BeginPlay: Mob Character")
  ;[0.7865 0.1065 0.7201] event bus setup
  (bind _returnvalue (`|AddComponentByClass` "/Game/MMOKit/MMO_Logic/Blueprints/EventBuses/BP_MobEventBus.BP_MobEventBus_C"))
  (set `self.EventBus` _returnvalue)
  (`/Engine/EditorBlueprintResources/StandardMacros.Can Execute Cosmetic Events`
    (:`False`
      ;[0.4452 0.6332 1] BeginPlay: set up stats & ai component
      (`|ExecutionSequence`
        (:`then_0`
          (set `self.StartingTransform` (`self.GetTransform`)))
        (:`then_1`
          (bind _returnvalue_2 (`|AddComponentByClass` "/Game/MMOKit/MMO_Logic/Blueprints/Stats/BP_MobStatsComponent.BP_MobStatsComponent_C"))
          (set `self.StatsComp` _returnvalue_2)
          (bind _returnvalue_3 (`|AddComponentByClass` (`self.AiComponentClass`)))
          (`/Engine/EditorBlueprintResources/StandardMacros.IsValid` _returnvalue_3
            (:`Is Valid`
              (set `self.AiComponent` _returnvalue_3))
            (:`Is Not Valid`
              (`MmoUtilities.LogString` "Error: AiComponentClass on this mob is empty" "Verbosity_Normal" true true (struct :`R` 1.0 :`B` 0.02448 :`A` 1.0) 10.0))))
        (:`then_2`
          (set `/Game/MMOKit/MMO_Logic/Blueprints/Stats/BP_BaseStatsComponent.MaxHp` _hp _statscomp)
          (set `/Game/MMOKit/MMO_Logic/Blueprints/Stats/BP_BaseStatsComponent.CurHp` _hp _statscomp)
          (`/Game/MMOKit/MMO_Logic/Blueprints/BP_AbilitySystemComponent.AddAbility` (`self.AbilitySystemComponent`) (`self.DefaultAttackAbility`)))
        (:`then_3`
          (add `/Game/MMOKit/MMO_Logic/Blueprints/EventBuses/BP_CharacterEventBus.OnTargetChanged` (`self.EventBus`) (delegate `OnTargetChanged`)))
        (:`then_4`
          (bind _output_get (set `self.Reaction` (`.MobReaction_8_E7C751FB42EEAA788D57008C195BB7D3` (break `/Game/MMOKit/MMO_Logic/Blueprints/Struct/FStatsMob` (`self.StartingStats`)))))
          (set `self.InitialReaction` _output_get)
          (set `self.ReplicatedMobName` (`.MobName_2_D74F93684FB9F0AF58E834944BEEE9CD` (break `/Game/MMOKit/MMO_Logic/Blueprints/Struct/FStatsMob` (`self.StartingStats`)))))
        (:`then_5`
          (`self.SanityCheckForLoot`))))))

(event `SanityCheckForLoot`
  ;[0.4452 0.6332 1] Sanity check for loot (on begin play on Server)
  (bind _values (`BlueprintMapLibrary.Map_Values` (`.ItemChance_7_920AEACB49CE8E94D2CAD8B8BFEDD6AA` (break `/Game/MMOKit/MMO_Logic/Blueprints/Struct/FMobLoot` (`self.DroppableLoot`)))))
  (for _array_element _values
    (if (or (> _array_element 1.0) (< _array_element 0.0))
      (`MmoUtilities.LogString` (`KismetStringLibrary.Concat_StrStr` "Mob's loot sanity check failed: " (`KismetSystemLibrary.GetObjectName` self)) "Verbosity_Normal" true true (struct :`R` 1.0 :`B` 0.02448 :`A` 1.0) 5.0))))

(event `self.ReceiveTick`
  (params (DeltaSeconds :type "Float (single-precision)"))
  (`parent.ReceiveTick` DeltaSeconds))

(event `OnTargetChanged`
  (params (NewTarget :type "Character Object Reference"))
  (bind ((`WalkSpeed_27_B4ED4B7F4467BA5F8EDA16BA418DB696` _walkspeed) (`RunSpeed_26_7DDAD1874B5FF67DE51250A5E27EC5B2` _runspeed)) (break `/Game/MMOKit/MMO_Logic/Blueprints/Struct/FStatsMob` (`self.StartingStats`)))
  ;[0.4452 0.6332 1] BeginPlay: set up stats & ai component
  (bind _output_get (set `self.InCombat` (`KismetSystemLibrary.IsValid` NewTarget)))
  (set `CharacterMovementComponent.MaxWalkSpeed` (`KismetMathLibrary.SelectFloat` _runspeed _walkspeed _output_get) (`self.CharacterMovement`)))

(event `/Game/MMOKit/MMO_Logic/Blueprints/Interfaces/BPI_MobSpecific.OnPlayerEnteredAggro`
  (params (PlayerCharacter :type "Character Object Reference"))
  (if (`self.IsHostileMob`)
    (`/Game/MMOKit/MMO_Logic/Blueprints/EventBuses/BP_MobEventBus.OnPlayerEnterAggroRange` (`self.EventBus`) PlayerCharacter)))

(event `/Game/MMOKit/MMO_Logic/Blueprints/Interfaces/BPI_Character.Die`
  (params (Killer :type "Character Object Reference"))
  (bind _startingstats (`self.StartingStats`))
  ;[0.4452 0.6332 1] Die (extends BaseCharacter's function)
  (`parent.Die` Killer)
  (`|ExecutionSequence`
    (:`then_0`
      (bind _eventbus (message `/Game/MMOKit/MMO_Logic/Blueprints/Interfaces/BPI_PlayerController.GetPlayerControllerEventBus` (`self.GetController` Killer)))
      (`/Engine/EditorBlueprintResources/StandardMacros.IsValid` _eventbus
        (:`Is Valid`
          (`/Game/MMOKit/MMO_Logic/Blueprints/EventBuses/BP_PlayerControllerEventBus.AwardXP_Multicast` _eventbus (`.XP_17_0AFF2D1A4C9A8A7E45934594BDF5C78E` (break `/Game/MMOKit/MMO_Logic/Blueprints/Struct/FStatsMob` (`self.StartingStats`)))))))
    (:`then_1`
      (`self.DropLoot`))
    (:`then_2`
      (message `/Game/MMOKit/MMO_Logic/Blueprints/Interfaces/BPI_GameMode.SpawnMobAfterDelay` (`GameplayStatics.GetGameMode`) (`self.StartingTransform`) (`GameplayStatics.GetObjectClass` self) _startingstats (`.RespawnDelay_20_CAC5EF814E5B1F28E7BA68B7B3825E75` (break `/Game/MMOKit/MMO_Logic/Blueprints/Struct/FStatsMob` _startingstats)) (`self.DroppableLoot`) (`self.BTAsset`))
      (`KismetSystemLibrary.Delay` 15.0)
      (`self.K2_DestroyActor`))))

(event `/Game/MMOKit/MMO_Logic/Blueprints/Interfaces/BPI_MobSpecific.OnPlayerLeftAggro`
  (params (Leaver :type "Character Object Reference"))
  (if (`self.IsHostileMob`)
    (message `/Game/MMOKit/MMO_Logic/Blueprints/Interfaces/BPI_MobSpecific.OnPlayerLeftAggro` (`self.EventBus`) Leaver)))

(event `/Game/MMOKit/MMO_Logic/Blueprints/Interfaces/BPI_MobSpecific.AttackTarget`
  (bind _defaultattackability (`self.DefaultAttackAbility`))
  (bind _targetcharacter (`/Game/MMOKit/MMO_Logic/Blueprints/BP_AIComponent.TargetCharacter` (`self.AiComponent`)))
  (`/Engine/EditorBlueprintResources/StandardMacros.IsValid` _defaultattackability
    (:`Is Valid`
      (bind _alive (message `/Game/MMOKit/MMO_Logic/Blueprints/Interfaces/BPI_Character.IsAlive` _targetcharacter))
      (if _alive
        (`self.UseAbilityFromServer` _defaultattackability _targetcharacter (`self.GetTransform` _targetcharacter))
        (else
          (`/Game/MMOKit/MMO_Logic/Blueprints/BP_AIComponent.UpdateTarget` (`self.AiComponent`)))))
    (:`Is Not Valid`
      (`MmoUtilities.LogString` "Error: mob has no default attack ability!" "Verbosity_Normal" true true (struct :`R` 1.0 :`B` 0.02448 :`A` 1.0) 10.0))))

(fn `DropLoot`
  (locals (RolledLoot :type "Array of PrimaryAssetId Structure") (Amounts :type "Array of Integer") (RolledFloat :type "Float (double-precision)" :default 0.0))
  (bind _keys (`BlueprintMapLibrary.Map_Keys` (`.ItemChance_7_920AEACB49CE8E94D2CAD8B8BFEDD6AA` (break `/Game/MMOKit/MMO_Logic/Blueprints/Struct/FMobLoot` (`self.DroppableLoot`)))))
  (for _array_element _keys
    (bind _output_get (set `local.RolledFloat` (`KismetMathLibrary.RandomFloat`)))
    (if (>= _output_get (`BlueprintMapLibrary.Map_Find` (`.ItemChance_7_920AEACB49CE8E94D2CAD8B8BFEDD6AA` (break `/Game/MMOKit/MMO_Logic/Blueprints/Struct/FMobLoot` (`self.DroppableLoot`))) _array_element))
      (`KismetArrayLibrary.Array_Add` (`local.RolledLoot`) _array_element)
      (`KismetArrayLibrary.Array_Add` (`local.Amounts`) 1)))
  (if (> (`KismetArrayLibrary.Array_Length` (`local.RolledLoot`)) 0)
    (`|SpawnActorFromClass` "/Game/MMOKit/MMO_Logic/Blueprints/Interaction/BP_LootBag.BP_LootBag_C" (`self.GetTransform`) "AdjustIfPossibleButAlwaysSpawn" "OverrideRootScale" null (`local.RolledLoot`) (`local.Amounts`) null)
    (`MmoUtilities.LogString` "Dropped loot")))

(fn `GetBehaviorTree`
  (returns (BTAsset :type "BehaviorTree Object Reference"))
  (return (`self.BTAsset`)))

(fn `GetCharacterEventBus`
  (returns (CharacterEventBus :type "/Game/MMOKit/MMO_Logic/Blueprints/EventBuses/BP_CharacterEventBus Object Reference"))
  (return (`self.EventBus`)))

(fn `GetMaxMoveSpeed`
  (returns (MaxSpeed :type "Float (double-precision)"))
  (return (`.RunSpeed_26_7DDAD1874B5FF67DE51250A5E27EC5B2` (break `/Game/MMOKit/MMO_Logic/Blueprints/Struct/FStatsMob` (`self.StartingStats`)))))

(fn `GetMobEventBus`
  (returns (EventBus :type "/Game/MMOKit/MMO_Logic/Blueprints/EventBuses/BP_MobEventBus Object Reference"))
  (return (`self.EventBus`)))

(fn `GetMobInitialReaction`
  (returns (Reaction :type "/Game/MMOKit/MMO_Logic/Blueprints/Enums/EReaction Enum"))
  (return (`self.InitialReaction`)))

(fn `GetMobName`
  (returns (MobName :type Text))
  (return (`self.ReplicatedMobName`)))

(fn `GetReaction`
  (returns (Reaction :type "/Game/MMOKit/MMO_Logic/Blueprints/Enums/EReaction Enum"))
  (return (`self.Reaction`)))

(fn `GetStatsComponent`
  (returns (StatsComp :type "/Game/MMOKit/MMO_Logic/Blueprints/Stats/BP_BaseStatsComponent Object Reference"))
  (return (`self.StatsComp`)))

(fn `GetTarget`
  (returns (TargetCharacter :type "Character Object Reference"))
  (return null))

(fn `IsHostileMob`
  (returns (Hostile :type Boolean))
  (return (`|EnumEquality` (`.MobReaction_8_E7C751FB42EEAA788D57008C195BB7D3` (break `/Game/MMOKit/MMO_Logic/Blueprints/Struct/FStatsMob` (`self.StartingStats`))) "NewEnumerator2")))

(fn `IsPlayerCharacter`
  (returns (IsPlayer :type Boolean))
  (return false))

(fn `OnRep_ReplicatedMobName`
  (`self.UpdateName`))

(fn `RollForDamage`
  (returns (Dmg :type Integer))
  (bind ((`DmgMin_13_73F87E7648F05DEEB2EA5CB4A92405D3` _dmgmin) (`DmgMax_14_4899B3EF4863BED094E1F08DF2F0A873` _dmgmax)) (break `/Game/MMOKit/MMO_Logic/Blueprints/Struct/FStatsMob` (`self.StartingStats`)))
  (return (`KismetMathLibrary.RandomIntegerInRange` _dmgmin _dmgmax)))

(fn `SetBody`
  (params (NewMesh :type "SkeletalMesh Object Reference") (AnimBp :type "AnimInstance Class Reference") (Sex :type "/Game/MMOKit/MMO_Logic/Blueprints/Enums/ECreatureSex Enum" :default "NewEnumerator0") (CreRace :type "/Game/MMOKit/MMO_Logic/Blueprints/Enums/ECreatureRace Enum" :default "NewEnumerator2"))
  (returns (Changed :type Boolean))
  (bind _changed (`parent.SetBody` NewMesh AnimBp Sex CreRace))
  (return _changed))

(fn `UserConstructionScript`
  (`parent.UserConstructionScript`))