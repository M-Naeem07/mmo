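; BPFL_Lib is a small Blueprint function library of general helpers in the MMOKit logic folder.
; Two functions null-check their target before destroying a component or removing a widget from its parent.
; FindDiff copies two collections into sets and uses set difference to return, as an array, items in the old collection missing from the new one.
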(fn `DestroyComponentIfValid`
  (params (Component :type "ActorComponent Object Reference"))
  (`/Engine/EditorBlueprintResources/StandardMacros.IsValid` Component
    (:`Is Valid`
      (`ActorComponent.K2_DestroyComponent` Component))))

(fn `FindDiff`
  (params (OldCollection :type "Array of PrimaryAssetId Structure") (NewCollection :type "Array of PrimaryAssetId Structure"))
  (returns (AssetsToUnload :type "Array of PrimaryAssetId Structure"))
  (locals (OldCollectionAsSet :type "Set of PrimaryAssetId Structure") (NewCollectionAsSet :type "Set of PrimaryAssetId Structure"))
  (`BlueprintSetLibrary.Set_AddItems` (`local.OldCollectionAsSet`) OldCollection)
  (`BlueprintSetLibrary.Set_AddItems` (`local.NewCollectionAsSet`) NewCollection)
  (bind _result (`BlueprintSetLibrary.Set_Difference` (`local.OldCollectionAsSet`) (`local.NewCollectionAsSet`)))
  (bind _result_2 (`BlueprintSetLibrary.Set_ToArray` _result))
  (return _result_2))

(fn `RemoveIfValid`
  (params (Widget :type "Widget Object Reference"))
  (`/Engine/EditorBlueprintResources/StandardMacros.IsValid` Widget
    (:`Is Valid`
      (`Widget.RemoveFromParent` Widget))))