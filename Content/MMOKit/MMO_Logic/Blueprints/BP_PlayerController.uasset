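; Player controller for an MMO that manages a player's character, input, HUD and three camera modes (first-person, over-shoulder, WoW-style).
; The server passes client cookie and character ID to GameMode, spawns characters from JSON, and saves them on unpossess outside PIE.
; Server-created replicated event bus, inventory, equipment and arbitrager components hold shared state and events.
; Camera type selects Enhanced Input mappings and, with the equipped weapon, the default attack ability.
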(event Custom|ChangeCameraType
  (params (NewCameraType :type ECameraType%20Enum :default "NewEnumerator0"))
  ;[1 0.312 0.302] Change Camera Type: called on runtime when the camera changes
  ; Not called on BeginPlay!
  (bind _alive (Class|BPICharacter|IsAlive(Message) (Pawn|GetControlledPawn)))
  (if _alive
    (bind _output_get (Variables|Default|SetCameraType NewCameraType))
    (CallFunction|SetupInputControls)
    (Default|SetupComponents (CallFunction|GetBPCharacter))
    ;;[1 0.312 0.302] will update ability depending on camera, because WoW-style uses AttackSword_TargetBased, while FP/TP uses AttackSword_Targetless.
    (Default|CallOnCameraChanged _output_get)
    (bind _eventbus (CallFunction|GetPlayerControllerEventBus))
    (Default|CallOnCameraChanged _eventbus _output_get)
    (CallFunction|ChangeCameraTypeServer _output_get)
    ;[1 0.312 0.302] if we switch to WoW, shut off Menu Mode
    (if (and (Utilities|Enum|Equal(Enum) _output_get "NewEnumerator2") (Variables|Default|GetIsMenuMode))
      (CallFunction|ForceMenuMode false))))

(event Custom|ForceMenuMode
  (params (On :type Boolean))
  ;[0 0.859 1] Event from the Input System
  ;;[1 1 1] Menu Mode On/Off
  ;; Only triggered in 1/3 person
  (if (!= On (Variables|Default|GetIsMenuMode))
    (bind _isa (Utilities|FlowControl|FlipFlop)
      (:A
        _)
      (:B
        _))
    (Default|CallOnMenuModeToggle _isa)
    (Variables|Default|SetIsMenuMode _isa)))

(event Custom|Server_ProvideCookieAndCharID
  (params (Cookie :type String) (CharID :type Integer))
  ;[0.4452 0.6332 1] Having intercepted the normal spawning of a pawn for a player controller, we arrive in CustomPlayerStart
  (Class|BPIGameMode|GetCharacterforController(Message) (Game|GetGameMode) self Cookie CharID))

(event Custom|OnCharacterResurrected
  ;[1 0.312 0.302] On Character Resurrected
  (bind _cameratype (CallFunction|GetCameraType))
  (if (or (Utilities|Enum|Equal(Enum) _cameratype "NewEnumerator0") (Utilities|Enum|Equal(Enum) _cameratype "NewEnumerator1"))
    (CallFunction|ForceMenuMode false)))

(event Custom|ForceEquipment
  (params (Open :type Boolean))
  ;[0 0.859 1] Event from the Input System
  ;;[1 1 1] Inventory & Equipment On/Off
  ;; Only triggered in Wow Camera
  (if (!= Open (Variables|Default|GetIsEquipmentOpen))
    (bind _isa (Utilities|FlowControl|FlipFlop)
      (:A
        _)
      (:B
        _))
    (Default|CallOnEquipmentToggle _isa)
    (Variables|Default|SetIsEquipmentOpen _isa)))

(event Custom|DisplayWarning3
  ;[1 1 1] If launching PIE in incorrect net mode, display a warning
  (bind _returnvalue (UserInterface|CreateWidget "/Game/MMOKit/MMO_Logic/Widgets/WBP_EditorWarning3.WBP_EditorWarning3_C"))
  (UserInterface|Viewport|AddtoViewport _returnvalue 0))

(event Custom|DisplayWarning1
  ;[1 1 1] Editor only: display warning if user hasn't launched the persistence server
  (bind _returnvalue (Class|MmoUtilities|InPieWorld))
  (if _returnvalue
    (bind _returnvalue_2 (UserInterface|CreateWidget "/Game/MMOKit/MMO_Logic/Widgets/WBP_EditorWarning1.WBP_EditorWarning1_C"))
    (UserInterface|Viewport|AddtoViewport _returnvalue_2 0)))

(event Custom|DisplayWarning2
  ;[1 1 1] Editor only: display a warning if there's not enough characters (or any) in the DB
  ; It can happen either when there's NO characters
  ; Or when we only have e.g. 2 characters, but we launch 3 PIE windows
  (bind _returnvalue (Class|MmoUtilities|InPieWorld))
  (if _returnvalue
    (bind _returnvalue_2 (UserInterface|CreateWidget "/Game/MMOKit/MMO_Logic/Widgets/WBP_EditorWarning2.WBP_EditorWarning2_C"))
    (UserInterface|Viewport|AddtoViewport _returnvalue_2 0)))

(event Custom|SpawnHud
  ;[1 0.312 0.302] Create HUD - Client Only
  (bind _returnvalue (UserInterface|CreateWidget "/Game/MMOKit/MMO_Logic/Widgets/WBP_HUD.WBP_HUD_C"))
  (bind _output_get (Variables|Default|SetHUD _returnvalue))
  (UserInterface|Viewport|AddtoViewport _output_get 0))

(event Custom|SetupInputControls
  (bind _modifycontextoptions (Utilities|Struct|MakeModifyContextOptions false false))
  (bind _self self)
  (bind _returnvalue (PlayerController|LocalPlayerSubsystems|GetEnhancedInputLocalPlayerSubsystem _self))
  ;[1 0.312 0.302] SetupCameraTypeControls
  ; Called on BeginPlay and whenever the camera type changes
  (Class|EnhancedInputSubsystemInterface|ClearAllMappings _returnvalue)
  (Class|EnhancedInputSubsystemInterface|RemovePlayerMappableConfig _returnvalue "/Game/MMOKit/MMO_Logic/InputConfig/DefaultInputConfig.DefaultInputConfig" (Utilities|Struct|MakeModifyContextOptions false true))
  (Class|EnhancedInputSubsystemInterface|AddPlayerMappableConfig _returnvalue "/Game/MMOKit/MMO_Logic/InputConfig/DefaultInputConfig.DefaultInputConfig" _modifycontextoptions) ; Already has IMC_Universal with priority 1
  (Input|AddMappingContext _returnvalue (Utilities|Select :Index (Variables|Default|GetCameraType) :NewEnumerator0 "/Game/MMOKit/MMO_Logic/InputConfig/IMC_FirstPersonControls.IMC_FirstPersonControls" :NewEnumerator1 "/Game/MMOKit/MMO_Logic/InputConfig/IMC_OverShoulderControls.IMC_OverShoulderControls" :NewEnumerator2 "/Game/MMOKit/MMO_Logic/InputConfig/IMC_WowStyleControls.IMC_WowStyleControls") 0 _modifycontextoptions) ; IMC_Universal has priority 1\nCamera-specific IMC has priority 0
)

(event Custom|LootFromLootable
  (params (Lootable :type BPI%20Lootable%20Interface) (Item :type Primary%20Asset%20Id%20Structure) (Id :type Integer) (Amount :type Integer))
  ;[0.4452 0.6332 1] Loot from Lootable
  (Default|LootItem Lootable Item Id Amount self))

(event Custom|ChangeCameraTypeServer
  (params (NewCameraType :type ECameraType%20Enum :default "NewEnumerator0"))
  ;[0.4452 0.6332 1] Change camera type: server - updates default ability
  (Variables|Default|SetCameraType NewCameraType)
  (bind (_item _amount) (Class|BPIStorage|GetItem(Message) (Variables|Default|GetEquipmentComponent) 1))
  (CallFunction|UpdateDefaultAbility _amount _item)
  (Default|CallOnCameraChanged NewCameraType)
  (bind _eventbus (CallFunction|GetPlayerControllerEventBus))
  (Default|CallOnCameraChanged _eventbus NewCameraType))

(event Custom|Client_RequestCookieAndCharID
  (bind _returnvalue (Game|GetGameInstance))
  ;[1 0.312 0.302] Client provides cookie and charID to server
  (bind _cookie (Class|BPIGameInstance|GetCookie(Message) _returnvalue))
  (bind _charid (Class|BPIGameInstance|GetCharId(Message) _returnvalue))
  (CallFunction|ServerProvideCookieandCharID _cookie _charid))

(event Custom|ForceInventory
  (params (Open :type Boolean))
  ;[0 0.859 1] Event from the Input System
  ;;[1 1 1] Inventory & Equipment On/Off
  ;; Only triggered in Wow Camera
  (if (!= Open (Variables|Default|GetIsInventoryOpen))
    (bind _isa (Utilities|FlowControl|FlipFlop)
      (:A
        _)
      (:B
        _))
    (Default|CallOnInventoryToggle _isa)
    (Variables|Default|SetIsInventoryOpen _isa)))

(event Custom|OnCharacterDied
  ;[1 0.312 0.302] On Character Died
  (bind _cameratype (CallFunction|GetCameraType))
  (if (or (Utilities|Enum|Equal(Enum) _cameratype "NewEnumerator0") (Utilities|Enum|Equal(Enum) _cameratype "NewEnumerator1"))
    (CallFunction|ForceMenuMode true)))

(event Input|EnhancedActionEvents|EnhancedInputActionIA_Jump
  (params (ActionValue :type Boolean) (ElapsedSeconds :type Float%20%28double-precision%29) (TriggeredSeconds :type Float%20%28double-precision%29) (InputAction :type Input%20Action%20Object%20Reference :default "/Game/MMOKit/MMO_Logic/InputConfig/IA_Jump.IA_Jump"))
  ;[0 0.859 1] Event from the Input System
  ;;[1 1 1] Movement
  (:Started
    (Default|CallOnJump)))

(event Input|EnhancedActionEvents|EnhancedInputActionIA_Jog
  (params (ActionValue :type Vector%202D%20Structure) (ElapsedSeconds :type Float%20%28double-precision%29) (TriggeredSeconds :type Float%20%28double-precision%29) (InputAction :type Input%20Action%20Object%20Reference :default "/Game/MMOKit/MMO_Logic/InputConfig/IA_Jog.IA_Jog"))
  ;[0 0.859 1] Event from the Input System
  ;;[1 1 1] Movement
  (:Triggered
    (Default|CallOnJog ActionValue))
  (:Started
    (Default|CallOnJogStart))
  (:Completed
    (Default|CallOnJogEnd)))

(event Input|EnhancedActionEvents|EnhancedInputActionIA_Equipment
  (params (ActionValue :type Boolean) (ElapsedSeconds :type Float%20%28double-precision%29) (TriggeredSeconds :type Float%20%28double-precision%29) (InputAction :type Input%20Action%20Object%20Reference :default "/Game/MMOKit/MMO_Logic/InputConfig/IA_Equipment.IA_Equipment"))
  ;[0 0.859 1] Event from the Input System
  ;;[1 1 1] Inventory & Equipment On/Off
  ;; Only triggered in Wow Camera
  (:Started
    (bind _isa (Utilities|FlowControl|FlipFlop)
      (:A
        _)
      (:B
        _))
    (Default|CallOnEquipmentToggle _isa)
    (Variables|Default|SetIsEquipmentOpen _isa)))

(event Input|EnhancedActionEvents|EnhancedInputActionIA_Enter
  (params (ActionValue :type Boolean) (ElapsedSeconds :type Float%20%28double-precision%29) (TriggeredSeconds :type Float%20%28double-precision%29) (InputAction :type Input%20Action%20Object%20Reference :default "/Game/MMOKit/MMO_Logic/InputConfig/IA_Enter.IA_Enter"))
  ;[0 0.859 1] Event from the Input System
  ;;[1 1 1] Enter key
  ;; (focus chat)
  (:Started
    (Default|CallOnFocusChat (Variables|Default|GetEventBus) true)))

(event Input|EnhancedActionEvents|EnhancedInputActionIA_LookAround
  (params (ActionValue :type Vector%202D%20Structure) (ElapsedSeconds :type Float%20%28double-precision%29) (TriggeredSeconds :type Float%20%28double-precision%29) (InputAction :type Input%20Action%20Object%20Reference :default "/Game/MMOKit/MMO_Logic/InputConfig/IA_LookAround.IA_LookAround"))
  ;[0 0.859 1] Event from the Input System
  ;;[1 1 1] LookAround / TurnAround
  ;;;[1 1 1] Depending on CameraType, IA_LookAround will be triggered by different keys (RMB + MouseLook or LMB + MouseLook in WowStyleCameraComponent, or just MouseLook in other camera types)
  (:Triggered
    (Default|CallOnLookAround ActionValue)))

(event Input|EnhancedActionEvents|EnhancedInputActionIA_RMB
  (params (ActionValue :type Boolean) (ElapsedSeconds :type Float%20%28double-precision%29) (TriggeredSeconds :type Float%20%28double-precision%29) (InputAction :type Input%20Action%20Object%20Reference :default "/Game/MMOKit/MMO_Logic/InputConfig/IA_RMB.IA_RMB"))
  ;[0 0.859 1] Event from the Input System
  ;;[1 1 1] LMB/RMB
  (:Started
    (Default|CallOnRmbDown ActionValue :!label _label))
  (:Completed
    (goto _label)))

(event Input|EnhancedActionEvents|EnhancedInputActionIA_TurnAround
  (params (ActionValue :type Float%20%28double-precision%29) (ElapsedSeconds :type Float%20%28double-precision%29) (TriggeredSeconds :type Float%20%28double-precision%29) (InputAction :type Input%20Action%20Object%20Reference :default "/Game/MMOKit/MMO_Logic/InputConfig/IA_TurnAround.IA_TurnAround"))
  ;[0 0.859 1] Event from the Input System
  ;;[1 1 1] LookAround / TurnAround
  ;;;[1 1 1] Depending on CameraType, IA_LookAround will be triggered by different keys (RMB + MouseLook or LMB + MouseLook in WowStyleCameraComponent, or just MouseLook in other camera types)
  (:Triggered
    (Default|CallOnTurnAround ActionValue)))

(event Input|EnhancedActionEvents|EnhancedInputActionIA_LMB
  (params (ActionValue :type Boolean) (ElapsedSeconds :type Float%20%28double-precision%29) (TriggeredSeconds :type Float%20%28double-precision%29) (InputAction :type Input%20Action%20Object%20Reference :default "/Game/MMOKit/MMO_Logic/InputConfig/IA_LMB.IA_LMB"))
  ;[0 0.859 1] Event from the Input System
  ;;[1 1 1] LMB/RMB
  (:Started
    (Default|CallOnLmbDown ActionValue :!label _label))
  (:Completed
    (goto _label)))

(event Input|EnhancedActionEvents|EnhancedInputActionIA_ZoomInOut
  (params (ActionValue :type Float%20%28double-precision%29) (ElapsedSeconds :type Float%20%28double-precision%29) (TriggeredSeconds :type Float%20%28double-precision%29) (InputAction :type Input%20Action%20Object%20Reference :default "/Game/MMOKit/MMO_Logic/InputConfig/IA_ZoomInOut.IA_ZoomInOut"))
  ;[0 0.859 1] Event from the Input System
  ;;[1 1 1] Zoom In/Out
  (:Triggered
    (Default|CallOnZoominOut ActionValue)))

(event Input|EnhancedActionEvents|EnhancedInputActionIA_Interact
  (params (ActionValue :type Boolean) (ElapsedSeconds :type Float%20%28double-precision%29) (TriggeredSeconds :type Float%20%28double-precision%29) (InputAction :type Input%20Action%20Object%20Reference :default "/Game/MMOKit/MMO_Logic/InputConfig/IA_Interact.IA_Interact"))
  ;[0 0.859 1] Event from the Input System
  ;;[1 1 1] Interact
  ;; In 1/3 person, turns off menu-mode if it's on
  (:Started
    (if (Variables|Default|GetIsMenuMode)
      (CallFunction|ForceMenuMode false)
      (else
        (Default|CallOnInteract)))))

(event Input|EnhancedActionEvents|EnhancedInputActionIA_MenuMode
  (params (ActionValue :type Boolean) (ElapsedSeconds :type Float%20%28double-precision%29) (TriggeredSeconds :type Float%20%28double-precision%29) (InputAction :type Input%20Action%20Object%20Reference :default "/Game/MMOKit/MMO_Logic/InputConfig/IA_MenuMode.IA_MenuMode"))
  ;[0 0.859 1] Event from the Input System
  ;;[1 1 1] Menu Mode On/Off
  ;; Only triggered in 1/3 person
  (:Started
    (bind _isa (Utilities|FlowControl|FlipFlop)
      (:A
        _)
      (:B
        _))
    (Default|CallOnMenuModeToggle _isa)
    (Variables|Default|SetIsMenuMode _isa)))

(event Input|EnhancedActionEvents|EnhancedInputActionIA_Inventory
  (params (ActionValue :type Boolean) (ElapsedSeconds :type Float%20%28double-precision%29) (TriggeredSeconds :type Float%20%28double-precision%29) (InputAction :type Input%20Action%20Object%20Reference :default "/Game/MMOKit/MMO_Logic/InputConfig/IA_Inventory.IA_Inventory"))
  ;[0 0.859 1] Event from the Input System
  ;;[1 1 1] Inventory & Equipment On/Off
  ;; Only triggered in Wow Camera
  (:Started
    (bind _isa (Utilities|FlowControl|FlipFlop)
      (:A
        _)
      (:B
        _))
    (Default|CallOnInventoryToggle _isa)
    (Variables|Default|SetIsInventoryOpen _isa)))

(event EventCustomPlayerStart
  ;[0.4452 0.6332 1] Having intercepted the normal spawning of a pawn for a player controller, we arrive in CustomPlayerStart
  (CallFunction|ClientRequestCookieandCharID))

(event EventUnPossess
  (params (UnpossessedPawn :type Pawn%20Object%20Reference))
  ;[0.4452 0.6332 1] In Game, OnUnPossess will save character to DB, but not in PIE
  ; In PIE, it gets destroyed too fast, so if we want to save a character, we have to do it manually
  (bind _returnvalue (Class|MmoUtilities|InPieWorld))
  (if (not _returnvalue)
    (Networking|CanExecuteCosmeticEvents
      (:False
        (CallFunction|SaveCharacter UnpossessedPawn)
        (bind _statscomp (Class|BPIStats|GetStatsComponent(Message) UnpossessedPawn))
        (bind _creaturename (Default|GetName _statscomp))
        (Class|BPIGameMode|CharacterLeftWorld(Message) (Game|GetGameMode) (Utilities|String|ToString(Text) _creaturename))))))

(event EventForceSaveCharacter
  ;[0.4452 0.6332 1] In Game, OnUnPossess will save character to DB, but not in PIE
  ; In PIE, it gets destroyed too fast, so if we want to save a character, we have to do it manually
  (Networking|CanExecuteCosmeticEvents
    (:False
      (CallFunction|SaveCharacter (Pawn|GetControlledPawn)))))

(event EventChatLostFocus
  ;[0 0.859 1] Event from the Input System
  ;;[1 1 1] On Chat Lost Focus
  (Default|CallOnChatLostFocus))

(event EventBeginPlay
  ;[1 1 1] BeginPlay: Assign mappable config,
  ; set default camera type
  (Class|MmoUtilities|LogString "BeginPlay: Controller" "Verbosity_SuperVerbose")
  (Networking|CanExecuteCosmeticEvents
    (:True
      (Utilities|IsValid (Variables|Default|GetEventBus) :!label _label
        (:Is%20Valid
          (CallFunction|SpawnHud)
          (CallFunction|SetupInputControls))
        (:Is%20Not%20Valid
          (Utilities|FlowControl|DelayUntilNextTick)
          (goto _label))))))

(event EventDisplayEditorWarning1
  ;[1 1 1] Editor only: display warning if user hasn't launched the persistence server
  (CallFunction|DisplayWarning1))

(event EventDisplayEditorWarning2
  ;[1 1 1] Editor only: display a warning if there's not enough characters (or any) in the DB
  ; It can happen either when there's NO characters
  ; Or when we only have e.g. 2 characters, but we launch 3 PIE windows
  (CallFunction|DisplayWarning2))

(event EventDisplayEditorWarning3
  ;[1 1 1] If launching PIE in incorrect net mode, display a warning
  (CallFunction|DisplayWarning3))

(event Input|KeyboardEvents|DebugKeyF1
  (params (Key :type Key%20Structure :default "None") (ActionValue :type Input%20Action%20Value%20Structure))
  ;[0 0.859 1] Event from the Input System
  ;;[1 1 1] DebugKeys F1-F3: FPS 30, 60, 120
  (:Pressed
    (Development|ExecuteConsoleCommand "t.MaxFPS 30" 0)))

(event Input|KeyboardEvents|DebugKeyF2
  (params (Key :type Key%20Structure :default "None") (ActionValue :type Input%20Action%20Value%20Structure))
  ;[0 0.859 1] Event from the Input System
  ;;[1 1 1] DebugKeys F1-F3: FPS 30, 60, 120
  (:Pressed
    (Development|ExecuteConsoleCommand "t.MaxFPS 60" 0)))

(event Input|KeyboardEvents|DebugKeyF3
  (params (Key :type Key%20Structure :default "None") (ActionValue :type Input%20Action%20Value%20Structure))
  ;[0 0.859 1] Event from the Input System
  ;;[1 1 1] DebugKeys F1-F3: FPS 30, 60, 120
  (:Pressed
    (Development|ExecuteConsoleCommand "t.MaxFPS 120" 0)))

(event Input|KeyboardEvents|F5
  (params (Key :type Key%20Structure :default "None"))
  ;[0 0.859 1] Event from the Input System
  ;;[1 1 1] DebugKeys F5-F7: Camera
  ;; FPS/TPS/WOW
  (:Pressed
    (CallFunction|ChangeCameraType "NewEnumerator0")))

(event Input|KeyboardEvents|F6
  (params (Key :type Key%20Structure :default "None"))
  ;[0 0.859 1] Event from the Input System
  ;;[1 1 1] DebugKeys F5-F7: Camera
  ;; FPS/TPS/WOW
  (:Pressed
    (CallFunction|ChangeCameraType "NewEnumerator1")))

(event Input|KeyboardEvents|F7
  (params (Key :type Key%20Structure :default "None"))
  ;[0 0.859 1] Event from the Input System
  ;;[1 1 1] DebugKeys F5-F7: Camera
  ;; FPS/TPS/WOW
  (:Pressed
    (CallFunction|ChangeCameraType "NewEnumerator2")))

(fn ConstructionScript
  ;[0.4452 0.6332 1] Initializes replicated components
  (Networking|CanExecuteCosmeticEvents
    (:False
      (bind _returnvalue (AddComponent|AddBPPlayerControllerEventBus))
      (Variables|Default|SetEventBus _returnvalue)
      (bind _returnvalue_2 (AddComponent|AddBPGridInventoryComponent))
      (Variables|Default|SetInventoryComponent _returnvalue_2) ; Note that the InventoryComponent variable is set to "Replicated", which means the same component will be added on client\nThe same applies to other "component" variables
      (bind _returnvalue_3 (AddComponent|AddBPEquipmentComponent))
      (Variables|Default|SetEquipmentComponent _returnvalue_3)
      (bind _returnvalue_4 (AddComponent|AddBPArbitragerComponent))
      (Variables|Default|SetArbitragerComponent _returnvalue_4))))

(fn IsRmbDown
  (return (Input|EnhancedActionValues|GetIA_RMB)))

(fn IsLmbDown
  (return (Input|EnhancedActionValues|GetIA_LMB)))

(fn GetIALookAround
  (return (Input|EnhancedActionValues|GetIA_LookAround)))

(fn GetIsJogging
  (return (not (Class|KismetMathLibrary|IsZero2D (Input|EnhancedActionValues|GetIA_Jog)))))

(fn GetIaTurnAround
  (return (Math|Conversions|ToFloat(Integer) (Input|EnhancedActionValues|GetIA_TurnAround))))

(fn GetBPCharacter
  (return (.AsBP%20Player%20Character (Utilities|Casting|CastToBP_PlayerCharacter (Pawn|GetControlledPawn)))))

(fn OnRepEquipmentComponent
  (EventDispatchers|BindEventtoOnRhandUpdated (Variables|Default|GetEquipmentComponent) (EventDispatchers|CreateEvent :!event UpdateDefaultAbility)))

(fn UpdateDefaultAbility
  (params (Amount :type Integer) (Weapon :type Primary%20Asset%20Id%20Structure))
  (bind _character (CallFunction|GetBPCharacter))
  ;[0.4452 0.6332 1] Called from: Equipment's OnRhandUpdate event, then from OnRep_EquipmentComponent
  ; Server function
  ; Also called when camera changes!
  (Networking|CanExecuteCosmeticEvents
    (:False
      (Utilities|FlowControl|Sequence
        (:then_0
          (LocalVariables|SetCachedDefaultAbility (Variables|Abilities|GetDefaultAbility)))
        (:then_1
          (if (> Amount 0)
            (bind _asequipment_asset (Utilities|Casting|CastToEquipmentAsset (Class|KismetSystemLibrary|GetObjectfromPrimaryAssetId Weapon))
              (:then
                (bind (_weaponstats _found) (Default|GetWeaponStats _asequipment_asset))
                (if _found
                  (Variables|Abilities|SetDefaultAbility (Utilities|Select :Index (Variables|/Game/MMOKit/MMO_Logic/Blueprints/DataAssetTypes/ItemProperties/WeaponStat.WeaponStat_C|GetBattleStance _weaponstats) :NewEnumerator0 0 :NewEnumerator1 (Utilities|Select :Index (Variables|Default|GetCameraType) :NewEnumerator0 "/Game/MMOKit/MMO_Content/Abilities/SwordAttack_Targetless.SwordAttack_Targetless" :NewEnumerator1 "/Game/MMOKit/MMO_Content/Abilities/SwordAttack_Targetless.SwordAttack_Targetless" :NewEnumerator2 "/Game/MMOKit/MMO_Content/Abilities/SwordAttack_TargetBased.SwordAttack_TargetBased")))
                  (else
                    (Variables|Abilities|SetDefaultAbility 0 :!label _label))))
              (:CastFailed
                (goto _label)))
            (else
              (goto _label))))
        (:then_2
          (if (!= (LocalVariables|GetCachedDefaultAbility) (Variables|Abilities|GetDefaultAbility))
            (Class|BPIAbilities|RemoveAbility(Message) _character (LocalVariables|GetCachedDefaultAbility))
            (Class|BPIAbilities|AddAbility(Message) _character (Variables|Abilities|GetDefaultAbility))))))))

(fn OnRepEventBus
  (bind _eventbus (Variables|Default|GetEventBus))
  (EventDispatchers|BindEventtoOnCharacterDied _eventbus (EventDispatchers|CreateEvent :!event Custom|OnCharacterDied))
  (EventDispatchers|BindEventtoOnCharacterResurrected _eventbus (EventDispatchers|CreateEvent :!event Custom|OnCharacterResurrected))
  (EventDispatchers|BindEventtoOnGotCharacterfromDB _eventbus (EventDispatchers|CreateEvent :!event SpawnCharacter)))

(fn SpawnCharacter
  (params (AccountID :type Integer) (CharID :type Integer) (CharName :type String) (Serialized :type String) (GuildID :type Integer) (GuildRank :type Integer))
  (bind _primaryassetid (Utilities|Struct|MakePrimaryAssetId))
  (Variables|Default|SetAccount%20ID AccountID)
  (Variables|Default|SetChar%20ID CharID)
  (Variables|Default|SetGuild%20ID GuildID)
  (Variables|Default|SetGuild%20Rank GuildRank)
  (Utilities|FlowControl|Sequence
    (:then_0
      (bind _outjsonobject (Class|JsonBlueprintFunctionLibrary|FromString Serialized))
      (bind _output_get (LocalVariables|SetJsonObj _outjsonobject))
      (bind _returnvalue (Class|JsonBlueprintFunctionLibrary|HasField _output_get "NewCharacter"))
      (if _returnvalue
        ;[0.4452 0.6332 1] Create new character if it's never been initialized
        (bind _outvalue (|GetJsonField (LocalVariables|GetJsonObj) "Sex"))
        (bind _outvalue_2 (|GetJsonField (LocalVariables|GetJsonObj) "Race"))
        (bind _outvalue_3 (|GetJsonField (LocalVariables|GetJsonObj) "RpgClass"))
        (bind _outactors (Actor|GetAllActorsOfClass "/Script/Engine.PlayerStart"))
        (bind _returnvalue_2 (Game|SpawnActorfromClass "/Game/MMOKit/MMO_Logic/Blueprints/BP_PlayerCharacter.BP_PlayerCharacter_C" (Transformation|GetActorTransform (Utilities|Array|Get(acopy) _outactors)) "Undefined" self (Utilities|Struct|MakeFStatsPlayer CharName 200 200 _outvalue_3) (Utilities|Struct|MakeFAppearancePartial _outvalue _outvalue_2) 0))
        (LocalVariables|SetSpawnedPlayerCharacter _returnvalue_2)
        (Class|MmoUtilities|LogString (Utilities|String|ToString(Text) (Utilities|Text|FormatText "Spawning player: {race}, {sex}, {rpgclass}" (Utilities|String|EnumtoString _outvalue_2) (Utilities|String|EnumtoString _outvalue) (Utilities|String|EnumtoString _outvalue_3))) "Verbosity_SuperVerbose")
        (Class|BPIGameMode|ContinuePlayerSpawn(Message) (Game|GetGameMode) self (LocalVariables|GetSpawnedPlayerCharacter) (.Rotation (Math|Transform|BreakTransform (Transformation|GetActorTransform (Utilities|Array|Get(acopy) _outactors))))) ; Will make Player Controller possess this character
        (Default|SignUptoControllerEvents (Variables|/Game/MMOKit/MMO_Logic/Blueprints/BP_BaseCharacter.BP_BaseCharacter_C|GetAppearanceComponent (LocalVariables|GetSpawnedPlayerCharacter)) (Variables|Default|GetEquipmentComponent))
        (Class|BPIGridInventoryComponent|Initialize(Message) (Variables|Default|GetInventoryComponent) (Utilities|Struct|MakeFGridInventory 64))
        (Default|Initialize (Variables|Default|GetEquipmentComponent) (Utilities|Struct|MakeFEquipment 3 (Utilities|Array|MakeArray _primaryassetid _primaryassetid _primaryassetid) (Utilities|Array|MakeArray 0 0 0)))
        (else
          ;[0.4452 0.6332 1] Restore character from db
          (bind _outvalue_4 (|GetJsonField (LocalVariables|GetJsonObj) "Stats"))
          (bind _outvalue_5 (|GetJsonField (LocalVariables|GetJsonObj) "Appearance"))
          (bind _outvalue_6 (|GetJsonField (LocalVariables|GetJsonObj) "Transform"))
          (bind _returnvalue_3 (Game|SpawnActorfromClass "/Game/MMOKit/MMO_Logic/Blueprints/BP_PlayerCharacter.BP_PlayerCharacter_C" _outvalue_6 "Undefined" self _outvalue_4 _outvalue_5 0))
          (bind _output_get_2 (LocalVariables|SetSpawnedPlayerCharacter _returnvalue_3))
          (Class|BPIGameMode|ContinuePlayerSpawn(Message) (Game|GetGameMode) self _output_get_2 (.Rotation (Math|Transform|BreakTransform _outvalue_6))) ; Will make Player Controller possess this character
          (Default|SignUptoControllerEvents (Variables|/Game/MMOKit/MMO_Logic/Blueprints/BP_BaseCharacter.BP_BaseCharacter_C|GetAppearanceComponent (LocalVariables|GetSpawnedPlayerCharacter)) (Variables|Default|GetEquipmentComponent))
          (bind _outvalue_7 (|GetJsonField (LocalVariables|GetJsonObj) "Inventory"))
          (Class|BPIGridInventoryComponent|Initialize(Message) (Variables|Default|GetInventoryComponent) _outvalue_7)
          (bind _outvalue_8 (|GetJsonField (LocalVariables|GetJsonObj) "Equipment"))
          (Default|Initialize (Variables|Default|GetEquipmentComponent) _outvalue_8))))
    (:then_1
      ;[0.4452 0.6332 1] after we've initialize character, add him to list of players in gamemode
      (Utilities|IsValid (LocalVariables|GetSpawnedPlayerCharacter)
        (:Is%20Valid
          (bind _statscomp (Default|GetStatsComponent (LocalVariables|GetSpawnedPlayerCharacter)))
          (bind _creaturename (Default|GetName _statscomp))
          (Class|BPIGameMode|CharacterEnteredWorld(Message) (Game|GetGameMode) (Utilities|String|ToString(Text) _creaturename) (LocalVariables|GetSpawnedPlayerCharacter)))))))

(fn SaveCharacter
  (params (ControlledPawn :type Pawn%20Object%20Reference))
  (LocalVariables|SetJsonObj (Utilities|Struct|MakeJsonObjectWrapper))
  (if (> (Variables|Default|GetChar%20ID) 0)
    (Utilities|IsValid ControlledPawn
      (:Is%20Valid
        (Utilities|FlowControl|Sequence
          (:then_0
            ;[1 1 1] Stats
            (bind _statscomp (Class|BPIStats|GetStatsComponent(Message) ControlledPawn))
            (bind _statsstruct (Class|BPIPlayerStats|GetSerializedStats(Message) _statscomp))
            (|SetJsonField (LocalVariables|GetJsonObj) "Stats" _statsstruct)
            ;[1 1 1] Appearance
            (bind _partialappearance (Class|BPIAppearance|GetPartialAppearance(Message) ControlledPawn))
            (|SetJsonField (LocalVariables|GetJsonObj) "Appearance" _partialappearance)
            ;[1 1 1] Transform
            (|SetJsonField (LocalVariables|GetJsonObj) "Transform" (Transformation|GetActorTransform ControlledPawn))
            ;[1 1 1] Inventory
            (bind _serializedinventory (Class|BPIGridInventoryComponent|GetSerializedInventory(Message) (Variables|Default|GetInventoryComponent)))
            (|SetJsonField (LocalVariables|GetJsonObj) "Inventory" _serializedinventory)
            ;[1 1 1] Equipment
            (bind _serializedequipment (Class|BPIEquipmentComponent|GetSerializedEquipment(Message) (Variables|Default|GetEquipmentComponent)))
            (|SetJsonField (LocalVariables|GetJsonObj) "Equipment" _serializedequipment))
          (:then_1
            (Class|BPIGameMode|SaveCharacter(Message) (Game|GetGameMode) (Variables|Default|GetChar%20ID) (LocalVariables|GetJsonObj)))))
      (:Is%20Not%20Valid
        (Class|MmoUtilities|LogString "Failed SaveCharToDb: pawn is null!" "Verbosity_Normal" true true "(R=1.000000,G=0.000000,B=0.024480,A=1.000000)")))
    (else
      (Class|MmoUtilities|LogString "Failed SaveCharToDb: character hasn't been set" "Verbosity_Normal" true true "(R=1.000000,G=0.000000,B=0.024480,A=1.000000)"))))

(fn GetCameraType
  (return (Variables|Default|GetCameraType)))

(fn GetCharId
  (return (Variables|Default|GetChar%20ID)))

(fn GetEquipmentSlot
  (params (Slot :type EEquipSlot%20Enum :default "NewEnumerator1"))
  (bind _returnvalue (Math|Conversions|ToInteger(Byte) Slot))
  (bind _equipmentcomponent (Variables|Default|GetEquipmentComponent))
  (bind _equipment (Variables|/Game/MMOKit/MMO_Logic/Blueprints/Inventory/BP_Equipment_Component.BP_Equipment_Component_C|GetEquipment _equipmentcomponent))
  (bind _output (Utilities|Array|Get(acopy) _equipment _returnvalue))
  (if (Utilities|Array|IsValidIndex _equipment _returnvalue)
    (if (AssetManager|IsValidPrimaryAssetId _output)
      (bind _asequipment_asset (Utilities|Casting|CastToEquipmentAsset (Class|KismetSystemLibrary|GetObjectfromPrimaryAssetId _output))
        (:then
          (return _asequipment_asset))
        (:CastFailed
          _))))
  (return 0))

(fn GetPlayerControllerEventBus
  (return (Variables|Default|GetEventBus)))