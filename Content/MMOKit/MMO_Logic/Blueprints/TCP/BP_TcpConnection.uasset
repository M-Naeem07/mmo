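; TCP connection to the MMO persistence server, used by game clients and servers for login, character data, chat and server travel.
; It reconnects on disconnect, sends periodic keep-alive probes, and logs in by cookie on clients or server password on servers outside StartMap.
; Requests are byte packets with an RPC enum and length-prefixed strings.
; A dispatch loop decodes replies and forwards them to event buses, GameInstance and GameMode.
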(event `ConnectToPersistenceServer`
  (bind _returnvalue (`MmoUtilities.CheckCommandLineParam` "local"))
  (bind _returnvalue_2 (`MmoUtilities.InPieWorld`))
  (bind _connectionid (`self.Connect` (`KismetMathLibrary.SelectString` "127.0.0.1" "107.152.143.34" (or _returnvalue_2 _returnvalue)) 3457 (delegate `OnDisconnect`) (delegate `OnConnect`) (`|CreateDelegate` :!event `On Message Received `)))
  (set `self.ConnectionId` _connectionid))

(event `OnDisconnect`
  (params (ConnectionId :type Integer))
  (`MmoUtilities.LogString` "Tcp Disconnect")
  (`KismetSystemLibrary.Delay` 1.0)
  (`self.ConnectToPersistenceServer`))

(event `OnConnect`
  (params (ConnectionId :type Integer))
  (`self.KeepAlive`)
  (`MmoUtilities.LogString` "Connected to persistence server")
  (bind _returnvalue (`GameplayStatics.GetCurrentLevelName` true))
  (if (not (== _returnvalue "StartMap"))
    (`self.Login`)))

(event `KeepAlive`
  ;[0.7865 0.1065 0.7201] Send KeepAlive probes once in a while, to prevent connection timeout, because you can't set KeepAlive in UE5 socket settings
  (`KismetSystemLibrary.K2_ClearAndInvalidateTimerHandle` (`self.KeepAliveTimer`))
  (bind _returnvalue (`KismetSystemLibrary.K2_SetTimerDelegate` (delegate `KeepAliveProbe`) 60.0 true))
  (set `self.KeepAliveTimer` _returnvalue))

(event `self.ReceiveEndPlay`
  (params (EndPlayReason :type "EEndPlayReason Enum" :default "Destroyed"))
  (bind _returnvalue (`MmoUtilities.InPieWorld`))
  (if _returnvalue
    (`/Engine/EditorBlueprintResources/StandardMacros.Can Execute Cosmetic Events`
      (:`False`
        (`MmoUtilities.LogString` "Tcp EndPlay")))))

(event `KeepAliveProbe`
  ;[0.7865 0.1065 0.7201] Send KeepAlive probes once in a while, to prevent connection timeout, because you can't set KeepAlive in UE5 socket settings
  (if (`self.isConnected` (`self.ConnectionId`))
    (`self.SendKeepAliveProbe`)))

(fn `CreateAccountResponse`
  (params (Message :type "Array of Byte"))
  (locals (Success :type Boolean))
  (`|ExecutionSequence`
    (:`then_0`
      (bind _returnvalue (`self.Message_ReadByte` Message)) ; read "success" bool
      (bind _output_get (set `local.Success` (> _returnvalue 0)))
      (if _output_get
        (bind _str (`self.ReadMmoString` Message))
        (message `/Game/MMOKit/MMO_Logic/Blueprints/Interfaces/BPI_GameInstance.SetCookie` (`GameplayStatics.GetGameInstance`) _str)))
    (:`then_1`
      (bind _eventbus (message `/Game/MMOKit/MMO_Logic/Blueprints/StartLevel/BPI_Start_PlayerController.GetStartEventBus` (`GameplayStatics.GetPlayerController` 0)))
      (`/Game/MMOKit/MMO_Logic/Blueprints/StartLevel/BP_Start_EventBus.OnCreateAccountResponse` _eventbus (`local.Success`)))))

(fn `CreateCharacter`
  (params (Charname :type String) (Sex :type "/Game/MMOKit/MMO_Logic/Blueprints/Enums/ECreatureSex Enum" :default "NewEnumerator0") (Race :type "/Game/MMOKit/MMO_Logic/Blueprints/Enums/ECreatureRace Enum" :default "NewEnumerator2") (ClassType :type "/Game/MMOKit/MMO_Logic/Blueprints/Enums/EClassType Enum" :default "NewEnumerator0"))
  (locals (JsonObj :type "JsonObjectWrapper Structure") (JsonString :type String) (NewCharacter :type Boolean :default true))
  (bind _jsonobj (`local.JsonObj`))
  (`|ExecutionSequence`
    (:`then_0`
      ;[1 0.312 0.302] We provide a flag "NewCharacter", which will tell the game server that it doesn't need to try deserializing anything other than a few fields, such as sex, race and rpgclass.
      ; The game server will create a stock level 1 character from these fields (race, sex, and class) and assign the level 1 inventory, stats, etc.
      ; And then the next time the character is saved, it will have its stats & equipment serialized. But not the first time.
      ; Note that this is the client that sends this. Which means the persistence server or the game server should do a sanity check.
      ; For example, a cheating client could send a forbidden combination of appearance and class, which we shouldn't allow. Or even invalid data, which we should reject.
      (set `local.JsonObj` (make `JsonObjectWrapper`))
      (`|SetJsonField` _jsonobj "Sex" (`KismetMathLibrary.Conv_ByteToInt` (`local.Sex`)))
      (`|SetJsonField` _jsonobj "Race" (`KismetMathLibrary.Conv_ByteToInt` (`local.Race`)))
      (`|SetJsonField` _jsonobj "RpgClass" (`KismetMathLibrary.Conv_ByteToInt` (`local.ClassType`)))
      (`|SetJsonField` _jsonobj "NewCharacter" (`local.NewCharacter`)))
    (:`then_1`
      (bind _outjsonstring (`JsonBlueprintFunctionLibrary.ToString` (`local.JsonObj`)))
      (bind _output_get (set `local.JsonString` _outjsonstring))
      (`MmoUtilities.LogString` (`KismetStringLibrary.Concat_StrStr` "Sending \"Create Character\" json: " _output_get)))
    (:`then_2`
      ;[1 0.312 0.302] The Persistence Server should also do a check on the name, because a cheating client could send something illegal, like a name a thousand characters long, which we should reject
      (`self.SendData` (`self.ConnectionId`) (`self.Concat_BytesBytes` (`self.CreateRpcEnum` "NewEnumerator20") (`self.CreateMmoString` Charname) (`self.CreateMmoString` (`local.JsonString`)))))))

(fn `CreateCharacterResponse`
  (params (Message :type "Array of Byte"))
  (bind _returnvalue (`self.Message_ReadByte` Message)) ; read "success" bool
  (bind _eventbus (message `/Game/MMOKit/MMO_Logic/Blueprints/StartLevel/BPI_Start_PlayerController.GetStartEventBus` (`GameplayStatics.GetPlayerController` 0)))
  (`/Game/MMOKit/MMO_Logic/Blueprints/StartLevel/BP_Start_EventBus.OnCreateCharacterResponse` _eventbus (> _returnvalue 0)))

(fn `CreateMmoString`
  (params (String :type String))
  (returns (Bytes :type "Array of Byte"))
  (bind _returnvalue (`self.Conv_StringToBytes` String))
  (return (`self.Concat_BytesBytes` (`self.Conv_IntToBytes` (`KismetArrayLibrary.Array_Length` _returnvalue)) _returnvalue)))

(fn `CreateRpcEnum`
  (params (Rpc :type "/Game/MMOKit/MMO_Logic/Blueprints/Enums/ERpcType Enum" :default "NewEnumerator0"))
  (returns (Bytes :type "Array of Byte"))
  (return (`self.Conv_ByteToBytes` Rpc)))

(fn `GetCharacter`
  (params (Cookie :type String) (CharID :type Integer))
  (`self.SendData` (`self.ConnectionId`) (`self.Concat_BytesBytes` (`self.CreateRpcEnum` "NewEnumerator23") (`self.CreateMmoString` Cookie) (`self.Conv_IntToBytes` CharID))))

(fn `GetCharacterResponse`
  (params (Message :type "Array of Byte"))
  (bind _message (`local.Message`))
  (bind _returnvalue (`self.Message_ReadByte` Message))
  (if (> _returnvalue 0)
    (bind _returnvalue_2 (`self.Message_ReadInt` _message))
    (bind _returnvalue_3 (`self.Message_ReadInt` _message))
    (bind _str (`self.ReadMmoString` _message))
    (bind _str_2 (`self.ReadMmoString` _message))
    (bind _returnvalue_4 (`self.Message_ReadInt` _message))
    (bind _returnvalue_5 (`self.Message_ReadInt` _message))
    (message `/Game/MMOKit/MMO_Logic/Blueprints/Interfaces/BPI_GameMode.GotCharacterForController` (`GameplayStatics.GetGameMode`) _returnvalue_2 _returnvalue_3 _str _str_2 _returnvalue_4 _returnvalue_5)
    (else
      (message `/Game/MMOKit/MMO_Logic/Blueprints/Interfaces/BPI_GameMode.FailedGettingCharacterForController` (`GameplayStatics.GetGameMode`)))))

(fn `GetCharacters`
  (`self.SendData` (`self.ConnectionId`) (`self.CreateRpcEnum` "NewEnumerator21")))

(fn `GetCharactersResponse`
  (params (Message :type "Array of Byte"))
  (locals (NumberOfCharacters :type Integer :default 0) (Names :type "Array of String") (Jsons :type "Array of String") (IDs :type "Array of Integer"))
  (bind _returnvalue (`self.Message_ReadInt` Message))
  (bind _output_get (set `local.NumberOfCharacters` _returnvalue))
  (for _ (range _output_get)
    (bind _returnvalue_2 (`self.Message_ReadInt` (`local.Message`)))
    (`KismetArrayLibrary.Array_Add` (`local.IDs`) _returnvalue_2)
    (bind _str (`self.ReadMmoString` (`local.Message`)))
    (`KismetArrayLibrary.Array_Add` (`local.Names`) _str)
    (bind _str_2 (`self.ReadMmoString` (`local.Message`)))
    (`KismetArrayLibrary.Array_Add` (`local.Jsons`) _str_2))
  (bind _eventbus (message `/Game/MMOKit/MMO_Logic/Blueprints/StartLevel/BPI_Start_PlayerController.GetStartEventBus` (`GameplayStatics.GetPlayerController` 0)))
  (`/Game/MMOKit/MMO_Logic/Blueprints/StartLevel/BP_Start_EventBus.OnGetCharactersResponse` _eventbus (`local.IDs`) (`local.Names`) (`local.Jsons`)))

(fn `GetIpAndPort`
  (params (CharId :type Integer))
  (`self.SendData` (`self.ConnectionId`) (`self.Concat_BytesBytes` (`self.CreateRpcEnum` "NewEnumerator22") (`self.Conv_IntToBytes` CharId))))

(fn `GetIpAndPortResponse`
  (params (Message :type "Array of Byte"))
  (bind _str (`self.ReadMmoString` Message))
  (`GameplayStatics.OpenLevel` (`KismetStringLibrary.Conv_StringToName` _str)))

(fn `KeepAliveAcknowledge`)

(fn `Login`
  (`/Engine/EditorBlueprintResources/StandardMacros.Can Execute Cosmetic Events`
    (:`True`
      ;[1 0.312 0.302] As client, send cookie and char id
      ; If in Editor, "GetCookie" and "GetCharId" it will provide a universal cookie instead, and PieWindowID respectively
      (bind _cookie (message `/Game/MMOKit/MMO_Logic/Blueprints/Interfaces/BPI_GameInstance.GetCookie` (`GameplayStatics.GetGameInstance`)))
      (bind _charid (message `/Game/MMOKit/MMO_Logic/Blueprints/Interfaces/BPI_GameInstance.GetCharId` (`GameplayStatics.GetGameInstance`)))
      (`self.SendData` (`self.ConnectionId`) (`self.Concat_BytesBytes` (`self.CreateRpcEnum` "NewEnumerator25") (`self.CreateMmoString` _cookie) (`self.Conv_IntToBytes` _charid))))
    (:`False`
      ;[0.4452 0.6332 1] As server, send password that is baked in only into server builds
      (bind _password (message `/Game/MMOKit/MMO_Logic/Blueprints/Interfaces/BPI_GameMode.GetServerPassword` (`GameplayStatics.GetGameMode`)))
      (`self.SendData` (`self.ConnectionId`) (`self.Concat_BytesBytes` (`self.CreateRpcEnum` "NewEnumerator24") (`self.CreateMmoString` _password))))))

(fn `LoginResponse`
  (params (Message :type "Array of Byte"))
  (locals (Success :type Boolean))
  (`|ExecutionSequence`
    (:`then_0`
      (bind _returnvalue (`self.Message_ReadByte` Message)) ; read "success" bool
      (bind _output_get (set `local.Success` (> _returnvalue 0)))
      (if _output_get
        (bind _str (`self.ReadMmoString` Message))
        (message `/Game/MMOKit/MMO_Logic/Blueprints/Interfaces/BPI_GameInstance.SetCookie` (`GameplayStatics.GetGameInstance`) _str)))
    (:`then_1`
      (bind _eventbus (message `/Game/MMOKit/MMO_Logic/Blueprints/StartLevel/BPI_Start_PlayerController.GetStartEventBus` (`GameplayStatics.GetPlayerController` 0)))
      (`/Game/MMOKit/MMO_Logic/Blueprints/StartLevel/BP_Start_EventBus.OnLoginResponse` _eventbus (`local.Success`)))))

(fn `LoginWithPassword`
  (params (Login :type String) (Password :type String))
  (`self.SendData` (`self.ConnectionId`) (`self.Concat_BytesBytes` (`self.CreateRpcEnum` "NewEnumerator3") (`self.CreateMmoString` Login) (`self.CreateMmoString` Password))))

(fn `LoginWithSteam`
  (params (SteamId :type String) (AuthTicket :type String))
  (`self.SendData` (`self.ConnectionId`) (`self.Concat_BytesBytes` (`self.CreateRpcEnum` "NewEnumerator18") (`self.CreateMmoString` SteamId) (`self.CreateMmoString` AuthTicket))))

(fn `MessageChannelRecieved`
  (params (Message :type "Array of Byte"))
  (`/Engine/EditorBlueprintResources/StandardMacros.Can Execute Cosmetic Events`
    (:`True`
      (bind _returnvalue (`self.Message_ReadInt` Message))
      (bind _str (`self.ReadMmoString` Message))
      (bind _str_2 (`self.ReadMmoString` Message))
      (bind _eventbus (message `/Game/MMOKit/MMO_Logic/Blueprints/Interfaces/BPI_PlayerController.GetPlayerControllerEventBus` (`GameplayStatics.GetPlayerController` 0)))
      (`/Game/MMOKit/MMO_Logic/Blueprints/EventBuses/BP_PlayerControllerEventBus.OnChannelMessage` _eventbus _returnvalue _str _str_2))
    (:`False`
      (bind _str_3 (`self.ReadMmoString` Message)) ; PlayerName
      (bind _str_4 (`self.ReadMmoString` Message)) ; Message
      (bind (_playerchar _found) (message `/Game/MMOKit/MMO_Logic/Blueprints/Interfaces/BPI_GameMode.GetPlayerCharByName` (`GameplayStatics.GetGameMode`) _str_3))
      (if _found
        (message `/Game/MMOKit/MMO_Logic/Blueprints/Interfaces/BPI_Character.Say` _playerchar _str_4)))))

(fn `MessagePlayerReceived`
  (params (Message :type "Array of Byte"))
  (bind _returnvalue (`self.Message_ReadByte` Message)) ; 0 means it's a message to ME\n1 means it's MY message that went through
  (bind _str (`self.ReadMmoString` Message)) ; Sender Name
  (bind _str_2 (`self.ReadMmoString` Message)) ; Message
  (bind _eventbus (message `/Game/MMOKit/MMO_Logic/Blueprints/Interfaces/BPI_PlayerController.GetPlayerControllerEventBus` (`GameplayStatics.GetPlayerController` 0)))
  (`/Game/MMOKit/MMO_Logic/Blueprints/EventBuses/BP_PlayerControllerEventBus.OnChannelMessage` _eventbus (`KismetMathLibrary.Conv_ByteToInt` (select `byte` _returnvalue :`0` "NewEnumerator2" :`1` "NewEnumerator5" :!type "/Game/MMOKit/MMO_Logic/Blueprints/Enums/EChatMsgChannel Enum")) _str _str_2))

(fn `NoSuchPlayer`
  (bind _eventbus (message `/Game/MMOKit/MMO_Logic/Blueprints/Interfaces/BPI_PlayerController.GetPlayerControllerEventBus` (`GameplayStatics.GetPlayerController` 0)))
  (`/Game/MMOKit/MMO_Logic/Blueprints/EventBuses/BP_PlayerControllerEventBus.OnChannelMessage` _eventbus (`KismetMathLibrary.Conv_ByteToInt` (enumliteral `/Game/MMOKit/MMO_Logic/Blueprints/Enums/EChatMsgChannel` "NewEnumerator4")) "" (`KismetTextLibrary.Conv_TextToString` "No such player!")))

(fn `On Message Received `
  (params (Connection :type Integer) (Message :type "Array of Byte"))
  (while (> (`KismetArrayLibrary.Array_Length` Message) 0)
    (bind _returnvalue (`self.Message_ReadByte` (`local.Message`)))
    (switch `/Game/MMOKit/MMO_Logic/Blueprints/Enums/ERpcType` (cast `/Game/MMOKit/MMO_Logic/Blueprints/Enums/ERpcType` _returnvalue)
      (:`NewEnumerator16`
        (`self.CreateAccountResponse` (`local.Message`)))
      (:`NewEnumerator3`
        (`self.LoginResponse` (`local.Message`)))
      (:`NewEnumerator18`
        (`self.SteamLoginResponse` (`local.Message`)))
      (:`NewEnumerator4`
        (`self.MessageChannelRecieved` (`local.Message`)))
      (:`NewEnumerator5`
        (`self.MessagePlayerReceived` (`local.Message`)))
      (:`NewEnumerator20`
        (`self.CreateCharacterResponse` (`local.Message`)))
      (:`NewEnumerator21`
        (`self.GetCharactersResponse` (`local.Message`)))
      (:`NewEnumerator22`
        (`self.GetIpAndPortResponse` (`local.Message`)))
      (:`NewEnumerator23`
        (`self.GetCharacterResponse` (`local.Message`)))
      (:`NewEnumerator27`
        (`self.NoSuchPlayer`))
      (:`NewEnumerator28`
        (`self.KeepAliveAcknowledge`)))))

(fn `ReadMmoString`
  (params (Message :type "Array of Byte"))
  (returns (Str :type String))
  (bind _returnvalue (`self.Message_ReadInt` Message))
  (if (> _returnvalue 0)
    (bind _returnvalue_2 (`self.Message_ReadString` Message _returnvalue))
    (return _returnvalue_2)
    (else
      (return ""))))

(fn `RegisterAccountWithPassword`
  (params (Account :type String) (Password :type String))
  (`self.SendData` (`self.ConnectionId`) (`self.Concat_BytesBytes` (`self.CreateRpcEnum` "NewEnumerator16") (`self.CreateMmoString` Account) (`self.CreateMmoString` Password))))

(fn `SaveCharacter`
  (params (CharId :type Integer) (JsonObj :type "JsonObjectWrapper Structure"))
  (bind (_outjsonstring _returnvalue) (`JsonBlueprintFunctionLibrary.ToString` JsonObj))
  (`MmoUtilities.LogString` _outjsonstring)
  (if _returnvalue
    (`self.SendData` (`self.ConnectionId`) (`self.Concat_BytesBytes` (`self.CreateRpcEnum` "NewEnumerator26") (`self.Conv_IntToBytes` CharId) (`self.CreateMmoString` _outjsonstring)))
    (`MmoUtilities.LogString` "Sending SaveCharacter")
    (else
      (`MmoUtilities.LogString` "Failed to save character: JsonObject to string failed" "Verbosity_Normal" true true (struct :`R` 1.0 :`B` 0.02448 :`A` 1.0) 5.0))))

(fn `SendChannelMessage`
  (params (Channel :type Integer) (Message :type String))
  (`self.SendData` (`self.ConnectionId`) (`self.Concat_BytesBytes` (`self.CreateRpcEnum` "NewEnumerator4") (`self.Conv_IntToBytes` Channel) (`self.CreateMmoString` (`self.TrimStringByLength` Message)))))

(fn `SendKeepAliveProbe`
  (`self.SendData` (`self.ConnectionId`) (`self.CreateRpcEnum` "NewEnumerator28")))

(fn `SendPrivateMessage`
  (params (Recipient :type String) (Message :type String))
  (`self.SendData` (`self.ConnectionId`) (`self.Concat_BytesBytes` (`self.CreateRpcEnum` "NewEnumerator5") (`self.CreateMmoString` Recipient) (`self.CreateMmoString` (`self.TrimStringByLength` Message)))))

(fn `SteamLoginResponse`
  (params (Message :type "Array of Byte"))
  (locals (Success :type Boolean))
  (`|ExecutionSequence`
    (:`then_0`
      (bind _returnvalue (`self.Message_ReadByte` Message)) ; read "success" bool
      (bind _output_get (set `local.Success` (> _returnvalue 0)))
      (if _output_get
        (bind _str (`self.ReadMmoString` Message))
        (message `/Game/MMOKit/MMO_Logic/Blueprints/Interfaces/BPI_GameInstance.SetCookie` (`GameplayStatics.GetGameInstance`) _str)
        (bind _eventbus (message `/Game/MMOKit/MMO_Logic/Blueprints/StartLevel/BPI_Start_PlayerController.GetStartEventBus` (`GameplayStatics.GetPlayerController` 0)))
        (`/Game/MMOKit/MMO_Logic/Blueprints/StartLevel/BP_Start_EventBus.OnLoginResponse` _eventbus true)
        (else
          (bind _str_2 (`self.ReadMmoString` Message))
          (bind _eventbus_2 (message `/Game/MMOKit/MMO_Logic/Blueprints/StartLevel/BPI_Start_PlayerController.GetStartEventBus` (`GameplayStatics.GetPlayerController` 0)))
          (`/Game/MMOKit/MMO_Logic/Blueprints/StartLevel/BP_Start_EventBus.OnSteamLoginFail` _eventbus_2 _str_2))))))

(fn `TrimStringByLength`
  (params (Original :type String))
  (returns (Shorter :type String))
  (if (> (`KismetStringLibrary.Len` Original) 0)
    (return (`KismetStringLibrary.GetSubstring` Original 0 (`self.StringMaxLength`)))
    (else
      (return (`local.Original`)))))

(fn `UserConstructionScript`)