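; Base storage component for the MMOKit inventory system, defining the slot-based interface that child storage classes override.
; Item queries, slot checks and removal are stubs that return false or empty results, and the content-updated event is an empty hook for subclasses.
; The only working logic is the MaxSlots RepNotify, which broadcasts the OnMaxSlotsChanged dispatcher with the new slot count.
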(event `EmitMaxSlotsChanged`
  (`self.OnMaxSlotsChanged` (`self.MaxSlots`)))

(event `EmitContentUpdated`)

(fn `AcceptsItem`
  (params (Item :type "PrimaryAssetId Structure") (Slot :type Integer))
  (returns (Accepts :type Boolean))
  (return false))

(fn `ContainsItem`
  (params (Slot :type Integer))
  (returns (Contains :type Boolean))
  (return false))

(fn `GetFirstAvailableSlot`
  (returns (Slot :type Integer) (HasAvailable :type Boolean))
  (return -1 false))

(fn `GetItem`
  (params (Slot :type Integer))
  (returns (Item :type "PrimaryAssetId Structure") (Amount :type Integer))
  (return (struct) 0))

(fn `IsSlotIdValid`
  (params (Slot :type Integer))
  (returns (Valid :type Boolean))
  (return false))

(fn `OnRep_MaxSlots`
  (`self.EmitMaxSlotsChanged`))

(fn `RemoveItem`
  (params (AtIndex :type Integer) (Silent :type Boolean))
  (returns (Success :type Boolean) (Item :type "PrimaryAssetId Structure") (Amount :type Integer))
  (return false (struct) 0))