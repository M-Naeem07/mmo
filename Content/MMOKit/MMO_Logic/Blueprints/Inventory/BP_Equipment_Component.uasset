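; Player controller component that holds a character's equipped head, right-hand and left-hand items as parallel asset ID and amount arrays.
; It implements inventory-style put, change and remove operations, blocked client-side with a log, and checks whether an item fits a slot.
; Changes are sent to the client for content updates and broadcast to drive appearance and the weapon-based attack ability.
; It initializes from database data and serializes back to an equipment struct.
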(event `OnEquipmentChanged`
  (bind _equipment (`self.Equipment`))
  ;[1 1 1] Replicate equipment to client
  (`self.SendToClient` (`self.Equipment`) (`self.Amounts`))
  (`self.OnAppearanceUpdated` (`|GetArrayItem` _equipment) (`|GetArrayItem` _equipment 1) (`|GetArrayItem` _equipment 2)) ; Bp_AppearanceComponent watches this event
  (`self.OnRhandUpdated` (`|GetArrayItem` (`self.Amounts`) 1) (`|GetArrayItem` (`self.Equipment`) 1)) ; Will update our Autoattack/LMB ability based on weapon
)

(event `self.EmitContentUpdated`
  ;[1 1 1] Emit content updated
  (bind _returnvalue (`|GenericCreateObject` "/Game/MMOKit/MMO_Logic/Blueprints/Inventory/BP_Equipment_UpdateData.BP_Equipment_UpdateData_C" (`self.Amounts`) (`self.Equipment`)))
  (`self.OnContentUpdated` _returnvalue))

(event `SendToClient`
  (params (Equipment :type "Array of PrimaryAssetId Structure") (Amounts :type "Array of Integer"))
  ;[1 1 1] Replicate equipment to client
  (set `self.Equipment` Equipment)
  (set `self.Amounts` Amounts)
  (`self.EmitContentUpdated`))

(event `self.ReceiveBeginPlay`
  ;[1 1 1] BeginPlay
  (bind _asbp_player_controller (cast `/Game/MMOKit/MMO_Logic/Blueprints/BP_PlayerController` (`self.GetOwner`))
    (:`then`
      (set `self.OwnerController` _asbp_player_controller))
    (:`CastFailed`
      (`MmoUtilities.LogString` "EquipComponent: must be attached to BP_PlayerController" "Verbosity_Normal" true true (struct :`R` 1.0 :`B` 0.02448 :`A` 1.0) 5.0))))

(event `Initialize`
  (params (InEquipment :type "/Game/MMOKit/MMO_Logic/Blueprints/Struct/FEquipment Structure"))
  (bind (_maxslots _equipment _amounts) (break `/Game/MMOKit/MMO_Logic/Blueprints/Struct/FEquipment` InEquipment))
  ;[0.4452 0.6332 1] Initialize is called from BP_PlayerController::SpawnCharacter which happens when we receive the character from DB
  (bind _output_get (set `self.MaxSlots` _maxslots))
  (set `self.Amounts` _amounts)
  (for _index (range _output_get)
    (bind _output (`|GetArrayItem` _equipment _index))
    (`KismetArrayLibrary.Array_Add` (`self.Equipment`) (select `bool` (`KismetSystemLibrary.IsValidPrimaryAssetId` _output) :`false` (make `PrimaryAssetId`) :`true` _output)))
  (`self.OnEquipmentChanged`))

(event `self.PutItem`
  (params (Slot :type Integer) (Item :type "PrimaryAssetId Structure") (Amount :type Integer))
  ;[1 1 1] Interface implementations
  (`/Engine/EditorBlueprintResources/StandardMacros.Can Execute Cosmetic Events`
    (:`True`
      (`MmoUtilities.LogString` "You're trying to PUT ITEM on the Client's Equipment. Only do it on the server!" "Verbosity_Normal" true true (struct :`R` 1.0 :`B` 0.02448 :`A` 1.0) 5.0))
    (:`False`
      (`self.PutItemOnServer` Slot Item Amount))))

(event `self.ChangeAmount`
  (params (AtIndex :type Integer) (NewAmount :type Integer))
  ;[1 1 1] Interface implementations
  (`/Engine/EditorBlueprintResources/StandardMacros.Can Execute Cosmetic Events`
    (:`True`
      (`MmoUtilities.LogString` "You're trying to CHANGE AMOUNT on the Client's Equipment. Only do it on the server!" "Verbosity_Normal" true true (struct :`R` 1.0 :`B` 0.02448 :`A` 1.0) 5.0))
    (:`False`
      (`self.ChangeAmountOnServer` AtIndex NewAmount))))

(event `self.AddItem`
  (params (Item :type "PrimaryAssetId Structure") (Amount :type Integer))
  ;[1 1 1] Interface implementations
  (`MmoUtilities.LogString` "Add Item is NOT a valid function for Equipment!" "Verbosity_Normal" true true (struct :`R` 1.0 :`B` 0.02448 :`A` 1.0) 5.0))

(fn `AcceptsItem`
  (params (Item :type "PrimaryAssetId Structure") (Slot :type Integer))
  (returns (Accepts :type Boolean))
  (bind _returnvalue (`KismetSystemLibrary.GetObjectFromPrimaryAssetId` Item))
  (`/Engine/EditorBlueprintResources/StandardMacros.IsValid` _returnvalue
    (:`Is Valid`
      (bind _asequipment_asset (cast `/Game/MMOKit/MMO_Logic/Blueprints/DataAssetTypes/EquipmentAsset` _returnvalue)
        (:`then`
          (bind _fits (`self.DoesEquipslotFit` (`/Game/MMOKit/MMO_Logic/Blueprints/DataAssetTypes/EquipmentAsset.Equip Slot` _asequipment_asset) Slot))
          (return _fits))
        (:`CastFailed`
          _)))
    (:`Is Not Valid`
      _))
  (`MmoUtilities.LogString` "EquipmentComponent: Accepts Item: problem" "Verbosity_Normal" true true (struct :`R` 1.0 :`B` 0.02448 :`A` 1.0))
  (return false))

(fn `ChangeAmountOnServer`
  (params (AtIndex :type Integer) (NewAmount :type Integer) (SendToClient :type Boolean :default true))
  (`|ExecutionSequence`
    (:`then_0`
      (bind _valid (`self.IsSlotIdValid` (`local.AtIndex`)))
      (if _valid
        (bind _contains (`self.ContainsItem` (`local.AtIndex`)))
        (if _contains
          (`|VariableSetRef` (`|GetArrayItem` (`self.Amounts`) (`local.AtIndex`)) (`local.NewAmount`))
          (if (<= (`local.NewAmount`) 0)
            (`|VariableSetRef` (`|GetArrayItem` (`self.Equipment`) (`local.AtIndex`)) (make `PrimaryAssetId`)))
          (else
            (`MmoUtilities.LogString` "Equipment: Change Amount failed (contains item was false)." "Verbosity_Normal" true true (struct :`R` 1.0 :`B` 0.02448 :`A` 1.0) 5.0)))
        (else
          (`MmoUtilities.LogString` "Equipment: Change Amount failed (slot invalid)" "Verbosity_Normal" true true (struct :`R` 1.0 :`B` 0.02448 :`A` 1.0) 5.0))))
    (:`then_1`
      (if SendToClient
        (`self.OnEquipmentChanged`)))))

(fn `ContainsItem`
  (params (Slot :type Integer))
  (returns (Contains :type Boolean))
  (if (and (`KismetArrayLibrary.Array_IsValidIndex` (`self.Amounts`) Slot) (`KismetArrayLibrary.Array_IsValidIndex` (`self.Equipment`) Slot))
    (return (> (`|GetArrayItem` (`self.Amounts`) (`local.Slot`)) 0))
    (else
      (return false))))

(fn `DoesEquipslotFit`
  (params (EquipSlot :type "/Game/MMOKit/MMO_Logic/Blueprints/Enums/EEquipSlot Enum" :default "NewEnumerator0") (EquipmentId :type Integer))
  (returns (Fits :type Boolean))
  ;[1 1 1] 0 = Head
  ; 1 = RightHand
  ; 2 = LeftHand
  ;
  ; If you have two ring slots next, it could be
  ; 3 = Ring
  ; 4 = Ring
  (switch `/Game/MMOKit/MMO_Logic/Blueprints/Enums/EEquipSlot` EquipSlot
    (:`NewEnumerator1`
      (return (== (`local.EquipmentId`) 0)))
    (:`NewEnumerator0`
      (return (== (`local.EquipmentId`) 1)))
    (:`NewEnumerator2`
      (return (== (`local.EquipmentId`) 2)))))

(fn `GetItem`
  (params (Slot :type Integer))
  (returns (Item :type "PrimaryAssetId Structure") (Amount :type Integer))
  (if (and (`KismetArrayLibrary.Array_IsValidIndex` (`self.Amounts`) Slot) (`KismetArrayLibrary.Array_IsValidIndex` (`self.Equipment`) Slot))
    (return (`|GetArrayItem` (`self.Equipment`) Slot) (`|GetArrayItem` (`self.Amounts`) Slot))
    (else
      (return (make `PrimaryAssetId`) 0))))

(fn `GetSerializedEquipment`
  (returns (SerializedEquipment :type "/Game/MMOKit/MMO_Logic/Blueprints/Struct/FEquipment Structure"))
  (return (make `/Game/MMOKit/MMO_Logic/Blueprints/Struct/FEquipment` (`self.MaxSlots`) (`self.Equipment`) (`self.Amounts`))))

(fn `GrowToAccomodateId`
  (params (SlotId :type Integer))
  (for _ (range (- (+ (`KismetArrayLibrary.Array_Length` (`self.Amounts`)) 1) SlotId))
    (`KismetArrayLibrary.Array_Add` (`self.Equipment`) (make `PrimaryAssetId`))
    (`KismetArrayLibrary.Array_Add` (`self.Amounts`))))

(fn `IsSlotIdValid`
  (params (Slot :type Integer))
  (returns (Valid :type Boolean))
  ;[1 1 1] For slot ID to be valid, it must be above or equal to 0, and less than MaxSlots
  (return (and (>= Slot 0) (< Slot (`self.MaxSlots`)))))

(fn `PutItemOnServer`
  (params (SlotId :type Integer) (Item :type "PrimaryAssetId Structure") (Amount :type Integer) (SendToClient :type Boolean :default true))
  (`|ExecutionSequence`
    (:`then_0`
      (bind _valid (`self.IsSlotIdValid` SlotId))
      (if (not _valid)
        (`self.GrowToAccomodateId` (`local.SlotId`)))
      (`|VariableSetRef` (`|GetArrayItem` (`self.Equipment`) (`local.SlotId`)) (`local.Item`))
      (`|VariableSetRef` (`|GetArrayItem` (`self.Amounts`) (`local.SlotId`)) (`local.Amount`)))
    (:`then_1`
      (if SendToClient
        (`self.OnEquipmentChanged`)))))

(fn `RemoveItem`
  (params (AtIndex :type Integer) (Silent :type Boolean))
  (returns (Success :type Boolean) (Item :type "PrimaryAssetId Structure") (Amount :type Integer))
  (locals (ReturnItem :type "PrimaryAssetId Structure") (ReturnAmount :type Integer))
  (`/Engine/EditorBlueprintResources/StandardMacros.Can Execute Cosmetic Events`
    (:`True`
      (`MmoUtilities.LogString` "Equipment: You're trying to REMOVE ITEM client-side! You must do it server-side!" "Verbosity_Normal" true true (struct :`R` 1.0 :`B` 0.02448 :`A` 1.0) 5.0))
    (:`False`
      (bind (_item _amount) (`self.GetItem` AtIndex))
      (if (> _amount 0)
        (set `local.ReturnItem` _item)
        (set `local.ReturnAmount` _amount)
        (`self.ChangeAmountOnServer` (`local.AtIndex`) 0 (not (`local.Silent`)))
        (return true (`local.ReturnItem`) (`local.ReturnAmount`))
        (else
          (return false (make `PrimaryAssetId`) 0))))))