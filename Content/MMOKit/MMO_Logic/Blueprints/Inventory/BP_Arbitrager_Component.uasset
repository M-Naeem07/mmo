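; Player controller component that arbitrates item moves, equips and unequips between inventory and equipment.
; It caches both storages as BPI_Storage on the non-cosmetic path, while cosmetic-capable instances route moves and unequips through request events to the server.
; MoveItemResolver validates slots, picks Move or Swap, checks AcceptsItem, then removes and re-puts items.
; As wired, Swap puts each item back in its original slot.
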(event `self.ReceiveBeginPlay`
  ;[1 1 1] BeginPlay: save a reference to inventory and equipment components
  (`/Engine/EditorBlueprintResources/StandardMacros.Can Execute Cosmetic Events`
    (:`False`
      (bind _asbp_player_controller (cast `/Game/MMOKit/MMO_Logic/Blueprints/BP_PlayerController` (`self.GetOwner`)))
      (`|ExecutionSequence`
        (:`then_0`
          (bind _inventorycomponent (`/Game/MMOKit/MMO_Logic/Blueprints/BP_PlayerController.InventoryComponent` _asbp_player_controller))
          (`/Engine/EditorBlueprintResources/StandardMacros.IsValid` _inventorycomponent
            (:`Is Valid`
              (if (`KismetSystemLibrary.DoesImplementInterface` _inventorycomponent "/Game/MMOKit/MMO_Logic/Blueprints/Inventory/BPI_Storage.BPI_Storage_C")
                (set `self.InventoryInterface` _inventorycomponent)
                (else
                  (`MmoUtilities.LogString` "Arbitrager: couldn't find inventory component" "Verbosity_Normal" true true (struct :`R` 1.0 :`B` 0.02448 :`A` 1.0) 5.0 :!label _label))))
            (:`Is Not Valid`
              (goto _label))))
        (:`then_1`
          (bind _equipmentcomponent (`/Game/MMOKit/MMO_Logic/Blueprints/BP_PlayerController.EquipmentComponent` _asbp_player_controller))
          (`/Engine/EditorBlueprintResources/StandardMacros.IsValid` _equipmentcomponent
            (:`Is Valid`
              (if (`KismetSystemLibrary.DoesImplementInterface` _equipmentcomponent "/Game/MMOKit/MMO_Logic/Blueprints/Inventory/BPI_Storage.BPI_Storage_C")
                (set `self.EquipmentInterface` _equipmentcomponent)
                (else
                  (`MmoUtilities.LogString` "Arbitrager: couldn't find equipment component" "Verbosity_Normal" true true (struct :`R` 1.0 :`B` 0.02448 :`A` 1.0) 5.0 :!label _label_2))))
            (:`Is Not Valid`
              (goto _label_2))))))))

(event `MoveItemRequest`
  (params (FromSlot :type Integer) (FromWindow :type "/Game/MMOKit/MMO_Logic/Blueprints/Enums/EItemsWindow Enum" :default "NewEnumerator0") (ToSlot :type Integer) (ToWindow :type "/Game/MMOKit/MMO_Logic/Blueprints/Enums/EItemsWindow Enum" :default "NewEnumerator0"))
  ;[0.4452 0.6332 1] MoveItemRequest
  (`self.MoveItemResolver` FromSlot FromWindow ToSlot ToWindow))

(event `MoveItem`
  (params (FromSlot :type Integer) (FromWindow :type "/Game/MMOKit/MMO_Logic/Blueprints/Enums/EItemsWindow Enum" :default "NewEnumerator0") (ToSlot :type Integer) (ToWindow :type "/Game/MMOKit/MMO_Logic/Blueprints/Enums/EItemsWindow Enum" :default "NewEnumerator0"))
  ;[1 1 1] MoveItem
  (`/Engine/EditorBlueprintResources/StandardMacros.Can Execute Cosmetic Events`
    (:`True`
      (`self.MoveItemRequest` FromSlot FromWindow ToSlot ToWindow))
    (:`False`
      (`self.MoveItemResolver` FromSlot FromWindow ToSlot ToWindow))))

(event `EquipItem`
  (params (FromSlot :type Integer) (FromWindow :type "/Game/MMOKit/MMO_Logic/Blueprints/Enums/EItemsWindow Enum" :default "NewEnumerator0") (ToSlot :type Integer))
  (`self.MoveItem` FromSlot FromWindow ToSlot "NewEnumerator1"))

(event `UnequipItem`
  (params (FromSlot :type Integer))
  ;[0.7865 0.1065 0.7201] Unequip Item
  (`/Engine/EditorBlueprintResources/StandardMacros.Can Execute Cosmetic Events`
    (:`True`
      (`self.RequestUnequip` FromSlot))
    (:`False`
      (`self.PerformUnequip` FromSlot))))

(event `RequestUnequip`
  (params (FromSlot :type Integer))
  ;[0.4452 0.6332 1] Request Unequip (server)
  (`self.PerformUnequip` FromSlot))

(event `PerformUnequip`
  (params (FromSlot :type Integer))
  ;[0.4452 0.6332 1] Peforms unequip on server
  (bind (_slot _hasavailable) (`/Game/MMOKit/MMO_Logic/Blueprints/Inventory/BPI_Storage.GetFirstAvailableSlot` (`self.InventoryInterface`)))
  (if _hasavailable
    (`self.MoveItem` FromSlot "NewEnumerator1" _slot)))

(fn `GetInterfaceObjectFromWindowType`
  (params (WindowType :type "/Game/MMOKit/MMO_Logic/Blueprints/Enums/EItemsWindow Enum" :default "NewEnumerator0"))
  (returns (ReturnValue :type "/Game/MMOKit/MMO_Logic/Blueprints/Inventory/BPI_Storage Interface"))
  (return (select `/Game/MMOKit/MMO_Logic/Blueprints/Enums/EItemsWindow` WindowType :`NewEnumerator0` (`self.InventoryInterface`) :`NewEnumerator1` (`self.EquipmentInterface`))))

(fn `MoveItemResolver`
  (params (FromSlot :type Integer) (FromWindow :type "/Game/MMOKit/MMO_Logic/Blueprints/Enums/EItemsWindow Enum" :default "NewEnumerator0") (ToSlot :type Integer) (ToWindow :type "/Game/MMOKit/MMO_Logic/Blueprints/Enums/EItemsWindow Enum" :default "NewEnumerator0"))
  (locals (Source :type "/Game/MMOKit/MMO_Logic/Blueprints/Inventory/BPI_Storage Interface") (Target :type "/Game/MMOKit/MMO_Logic/Blueprints/Inventory/BPI_Storage Interface") (OperationValidity :type Boolean) (OperationType :type "/Game/MMOKit/MMO_Logic/Blueprints/Enums/EArbitrageOperation Enum"))
  (`|ExecutionSequence`
    (:`then_0`
      ;[1 1 1] Input validity (check that item exists, that slot ids are valid, etc)
      (set `local.Source` (`self.GetInterfaceObjectFromWindowType` (`local.FromWindow`)))
      (set `local.Target` (`self.GetInterfaceObjectFromWindowType` (`local.ToWindow`)))
      (if (and (`|EnumEquality` (`local.ToWindow`) (`local.FromWindow`)) (== (`local.FromSlot`) (`local.ToSlot`)))
        (`MmoUtilities.LogString` "Arbitrager: Item move cancelled")
        (else
          (bind _valid (`/Game/MMOKit/MMO_Logic/Blueprints/Inventory/BPI_Storage.IsSlotIdValid` (`local.Target`) (`local.ToSlot`)))
          (bind _valid_2 (`/Game/MMOKit/MMO_Logic/Blueprints/Inventory/BPI_Storage.IsSlotIdValid` (`local.Source`) (`local.FromSlot`)))
          (bind _contains (`/Game/MMOKit/MMO_Logic/Blueprints/Inventory/BPI_Storage.ContainsItem` (`local.Source`) (`local.FromSlot`)))
          (if (and _contains _valid_2 _valid)
            (bind _contains_2 (`/Game/MMOKit/MMO_Logic/Blueprints/Inventory/BPI_Storage.ContainsItem` (`local.Target`) (`local.ToSlot`)))
            (if _contains_2
              ;;[1 1 1] If you want to do more than swap, e.g. work with stacks, this is where you'd set another type of operation
              (set `local.OperationType` "NewEnumerator1")
              (else
                (set `local.OperationType` "NewEnumerator0")))
            (else
              (`MmoUtilities.LogString` "Arbitrager: Input validity checks didn't pass" "Verbosity_Normal" true true (struct :`R` 1.0 :`B` 0.02448 :`A` 1.0)))))))
    (:`then_1`
      ;[1 1 1] Operation validity (check that items can fit to target slots, e.g. a helm can go into a head slot)
      (switch `/Game/MMOKit/MMO_Logic/Blueprints/Enums/EArbitrageOperation` (`local.OperationType`)
        (:`NewEnumerator0`
          (bind _item (`/Game/MMOKit/MMO_Logic/Blueprints/Inventory/BPI_Storage.GetItem` (`local.Source`) (`local.FromSlot`)))
          (bind _accepts (`/Game/MMOKit/MMO_Logic/Blueprints/Inventory/BPI_Storage.AcceptsItem` (`local.Target`) _item (`local.ToSlot`)))
          (set `local.OperationValidity` _accepts))
        (:`NewEnumerator1`
          (bind _item_2 (`/Game/MMOKit/MMO_Logic/Blueprints/Inventory/BPI_Storage.GetItem` (`local.Source`) (`local.FromSlot`)))
          (bind _accepts_2 (`/Game/MMOKit/MMO_Logic/Blueprints/Inventory/BPI_Storage.AcceptsItem` (`local.Target`) _item_2 (`local.ToSlot`)))
          (bind _item_3 (`/Game/MMOKit/MMO_Logic/Blueprints/Inventory/BPI_Storage.GetItem` (`local.Target`) (`local.ToSlot`)))
          (bind _accepts_3 (`/Game/MMOKit/MMO_Logic/Blueprints/Inventory/BPI_Storage.AcceptsItem` (`local.Source`) _item_3 (`local.FromSlot`)))
          (set `local.OperationValidity` (and _accepts_3 _accepts_2)))))
    (:`then_2`
      ;[1 1 1] Operation itself
      (if (`local.OperationValidity`)
        (switch `/Game/MMOKit/MMO_Logic/Blueprints/Enums/EArbitrageOperation` (`local.OperationType`)
          (:`NewEnumerator0`
            (bind (_success _item_4 _amount) (`/Game/MMOKit/MMO_Logic/Blueprints/Inventory/BPI_Storage.RemoveItem` (`local.Source`) (`local.FromSlot`) false))
            (if _success
              (`/Game/MMOKit/MMO_Logic/Blueprints/Inventory/BPI_Storage.PutItem` (`local.Target`) (`local.ToSlot`) _item_4 _amount)
              (else
                (`MmoUtilities.LogString` "Arbitrager: Move went wrong" "Verbosity_Normal" true true (struct :`R` 1.0 :`B` 0.02448 :`A` 1.0)))))
          (:`NewEnumerator1`
            (bind (_success_2 _item_5 _amount_2) (`/Game/MMOKit/MMO_Logic/Blueprints/Inventory/BPI_Storage.RemoveItem` (`local.Source`) (`local.FromSlot`) false))
            (bind (_success_3 _item_6 _amount_3) (`/Game/MMOKit/MMO_Logic/Blueprints/Inventory/BPI_Storage.RemoveItem` (`local.Target`) (`local.ToSlot`) false))
            (if (and _success_2 _success_3)
              (`/Game/MMOKit/MMO_Logic/Blueprints/Inventory/BPI_Storage.PutItem` (`local.Target`) (`local.ToSlot`) _item_6 _amount_3)
              (`/Game/MMOKit/MMO_Logic/Blueprints/Inventory/BPI_Storage.PutItem` (`local.Source`) (`local.FromSlot`) _item_5 _amount_2)
              (else
                (`MmoUtilities.LogString` "Arbitrager: Swap went wrong" "Verbosity_Normal" true true (struct :`R` 1.0 :`B` 0.02448 :`A` 1.0))))))
        (else
          (`MmoUtilities.LogString` "Arbitrager: Operation validity checks didn't pass" "Verbosity_Normal" true true (struct :`R` 1.0 :`B` 0.02448 :`A` 1.0)))))))