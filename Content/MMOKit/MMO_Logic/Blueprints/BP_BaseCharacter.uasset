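; Base character for players and mobs in the MMO kit, handling appearance, gear, abilities, melee traces and death.
; Forwards calls to its ability and appearance components, and reaches stats and event bus through getters that children override.
; Death and resurrection multicast to the event bus; replicated IsDead toggles collision and client-side ragdoll after the death montage.
; SetBody swaps mesh and attaches eyes; SetGear async-loads right-hand meshes.
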(event `SetNameplateWidget`
  ;[1 1 1] To Override by children classes
)

(event `UpdateName`
  ;[1 1 1] Update Name (called from OnRep Mob's RepMobName)
  (bind _statscomp (`/Game/MMOKit/MMO_Logic/Blueprints/Stats/BPI_Stats.GetStatsComponent` :!label _label))
  (`/Engine/EditorBlueprintResources/StandardMacros.IsValid` _statscomp
    (:`Is Valid`
      (`/Game/MMOKit/MMO_Logic/Blueprints/Stats/BP_BaseStatsComponent.EmitNameUpdated` _statscomp))
    (:`Is Not Valid`
      (`KismetSystemLibrary.DelayUntilNextTick`)
      (goto _label))))

(event `UpdateReaction`
  ;[1 0.312 0.302] Update Reaction (called from OnRep reaction)
  (bind _charactereventbus (`/Game/MMOKit/MMO_Logic/Blueprints/Interfaces/BPI_Character.GetCharacterEventBus`))
  (`/Engine/EditorBlueprintResources/StandardMacros.IsValid` _charactereventbus :!label _label_2
    (:`Is Valid`
      (`/Game/MMOKit/MMO_Logic/Blueprints/EventBuses/BP_CharacterEventBus.OnUpdateReaction` _charactereventbus (`self.Reaction`)))
    (:`Is Not Valid`
      (`KismetSystemLibrary.DelayUntilNextTick`)
      (goto _label_2))))

(event `self.ReceiveTick`
  (params (DeltaSeconds :type "Float (single-precision)"))
  ;[1 1 1] Tick
)

(event `self.ReceiveBeginPlay`
  (set `CharacterMovementComponent.MaxWalkSpeed` (`self.MaxMoveSpeed`) (`self.CharacterMovement`))
  (`/Engine/EditorBlueprintResources/StandardMacros.Can Execute Cosmetic Events`
    (:`True`
      ;[1 0.312 0.302] BeginPlay Client-side
      (`self.SetNameplateWidget`))))

(event `self.SetGear`
  (params (Head :type "PrimaryAssetId Structure") (RHand :type "PrimaryAssetId Structure") (LHand :type "PrimaryAssetId Structure"))
  (bind _rhandmeshcomponent (`self.RhandMeshComponent`))
  ;[1 0.312 0.302] SetGear
  (`|ExecutionSequence`
    (:`then_0`
      (bind _asequipment_asset (cast `/Game/MMOKit/MMO_Logic/Blueprints/DataAssetTypes/EquipmentAsset` (`KismetSystemLibrary.GetObjectFromPrimaryAssetId` RHand))
        (:`then`
          (bind _object (`|LoadAsset` (`/Game/MMOKit/MMO_Logic/Blueprints/DataAssetTypes/EquipmentAsset.StatMesh` _asequipment_asset))
            (:`Completed`
              (bind _asstatic_mesh (cast `StaticMesh` _object))
              (`/Engine/EditorBlueprintResources/StandardMacros.IsValid` _asstatic_mesh
                (:`Is Valid`
                  (`/Engine/EditorBlueprintResources/StandardMacros.IsValid` (`self.RhandMeshComponent`)
                    (:`Is Valid`
                      (`StaticMeshComponent.SetStaticMesh` _rhandmeshcomponent _asstatic_mesh :!label _label_3)
                      (`SceneComponent.SetVisibility` _rhandmeshcomponent (`SceneComponent.bVisible` (`self.Mesh`)) false))
                    (:`Is Not Valid`
                      (`/Engine/EditorBlueprintResources/StandardMacros.IsValid` (`SkeletalMeshComponent.GetSkeletalMeshAsset` (`self.Mesh`))
                        (:`Is Valid`
                          (bind _returnvalue (`|AddComponentByClass` "/Script/Engine.StaticMeshComponent" true))
                          (bind _output_get (set `self.RhandMeshComponent` _returnvalue))
                          (`PrimitiveComponent.SetCollisionEnabled` _output_get "NoCollision")
                          (`SceneComponent.K2_AttachToComponent` (`self.RhandMeshComponent`) (`self.Mesh`) "hand_rSocket" "SnapToTarget" "SnapToTarget" "SnapToTarget" true)
                          (goto _label_3))
                        (:`Is Not Valid`
                          (`MmoUtilities.LogString` "BaseCharacter: WOAH! This can never happen!" "Verbosity_Normal" true true (struct :`R` 1.0 :`B` 0.02448 :`A` 1.0)))))))
                (:`Is Not Valid`
                  (`/Game/MMOKit/MMO_Logic/Blueprints/BPFL_Lib.DestroyComponentIfValid` (`self.RhandMeshComponent`) :!label _label_4))))))
        (:`CastFailed`
          (goto _label_4))))))

(event `/Game/MMOKit/MMO_Logic/Blueprints/Interfaces/BPI_Abilities.AddAbility`
  (params (Ability :type "/Game/MMOKit/MMO_Logic/Blueprints/DataAssetTypes/AbilityAsset Object Reference"))
  ;[0.7865 0 0.7097] Ability Component Management
  (`/Game/MMOKit/MMO_Logic/Blueprints/BP_AbilitySystemComponent.AddAbility` (`self.AbilitySystemComponent`) Ability))

(event `/Game/MMOKit/MMO_Logic/Blueprints/Interfaces/BPI_Character.Resurrect`
  ;[0.4452 0.6332 1] Resurrect (server) - don't call directly,
  ; call StatsComponent's Resurrect
  (`self.Resurrect_Multicast`)
  (`CharacterMovementComponent.SetMovementMode` (`self.CharacterMovement`) "MOVE_Walking" 0))

(event `/Game/MMOKit/MMO_Logic/Blueprints/Interfaces/BPI_Abilities.RemoveAbility`
  (params (Ability :type "/Game/MMOKit/MMO_Logic/Blueprints/DataAssetTypes/AbilityAsset Object Reference"))
  ;[0.7865 0 0.7097] Ability Component Management
  (`/Game/MMOKit/MMO_Logic/Blueprints/BP_AbilitySystemComponent.AddAbility` (`self.AbilitySystemComponent`) Ability))

(event `self.SwapSex`
  ;[0.4452 0.6332 1] Swap sex
  (`/Game/MMOKit/MMO_Logic/Blueprints/BP_AppearanceComponent.SwapSex` (`self.AppearanceComponent`)))

(event `/Game/MMOKit/MMO_Logic/Blueprints/Interfaces/BPI_Abilities.UseAbility`
  (params (Ability :type "/Game/MMOKit/MMO_Logic/Blueprints/DataAssetTypes/AbilityAsset Object Reference"))
  ;[0.7865 0 0.7097] Ability Component Management
  (`/Game/MMOKit/MMO_Logic/Blueprints/BP_AbilitySystemComponent.ActivateAbilityFromClient` (`self.AbilitySystemComponent`) Ability))

(event `Resurrect_Multicast`
  ;[0.7865 0.1065 0.7201] Resurrect Multicast
  (set `self.IsDead` false)
  (bind _charactereventbus (`/Game/MMOKit/MMO_Logic/Blueprints/Interfaces/BPI_Character.GetCharacterEventBus`))
  (`/Game/MMOKit/MMO_Logic/Blueprints/EventBuses/BP_CharacterEventBus.OnResurrect` _charactereventbus))

(event `/Game/MMOKit/MMO_Logic/Blueprints/Interfaces/BPI_Character.Die`
  (params (Killer :type "Character Object Reference"))
  ;[0.4452 0.6332 1] Die (server) - don't call directly,
  ; rather do StatsComponent->TakeDamage
  (`self.Die_Multicast`)
  (`CharacterMovementComponent.DisableMovement` (`self.CharacterMovement`)))

(event `/Game/MMOKit/MMO_Logic/Blueprints/Interfaces/BPI_Abilities.UseAbilityFromServer`
  (params (Ability :type "/Game/MMOKit/MMO_Logic/Blueprints/DataAssetTypes/AbilityAsset Object Reference") (OptionalVictim :type "Character Object Reference") (OptionalInstigatorTransform :type "Transform Structure"))
  ;[0.7865 0 0.7097] Ability Component Management
  (`/Game/MMOKit/MMO_Logic/Blueprints/BP_AbilitySystemComponent.ActivateAbilityFromServer` (`self.AbilitySystemComponent`) Ability OptionalVictim OptionalInstigatorTransform))

(event `self.SwapSpecies`
  ;[0.4452 0.6332 1] Swap species
  (`/Game/MMOKit/MMO_Logic/Blueprints/BP_AppearanceComponent.SwapSpecies` (`self.AppearanceComponent`)))

(event `Die_Multicast`
  ;[0.7865 0.1065 0.7201] Die Multicast - extended in PlayerCharacter and MobCharacter
  (`PrimitiveComponent.SetCollisionProfileName` (`self.CapsuleComponent`) "PawnDead" true) ; Although OnRep_IsDead also sets collision profile, this is needed here too
  (bind _charactereventbus (`/Game/MMOKit/MMO_Logic/Blueprints/Interfaces/BPI_Character.GetCharacterEventBus`))
  (`/Game/MMOKit/MMO_Logic/Blueprints/EventBuses/BP_CharacterEventBus.OnDeath` _charactereventbus)
  (`/Engine/EditorBlueprintResources/StandardMacros.Can Execute Cosmetic Events`
    (:`True`
      ;[1 0.312 0.302] Ragdoll on client
      (`|PlayMontage` (`self.Mesh`) (`self.GetDeathMontage`)
        (:`OnBlendOut`
          ;;[1 0.312 0.302] ragdoll in OnRep_IsDead
          (set `self.IsDead` true))))
    (:`False`
      (`KismetSystemLibrary.Delay` (`AnimSequenceBase.SequenceLength` (`self.GetDeathMontage`)))
      (set `self.IsDead` true) ; ragdoll
    )))

(event `/Game/MMOKit/MMO_Logic/Blueprints/Interfaces/BPI_Character.Say`
  (params (Message :type String))
  (`self.SayClient` Message))

(event `SayClient`
  (params (Message :type String))
  (bind _returnvalue (`GameplayStatics.GetPlayerController` 0))
  (`/Engine/EditorBlueprintResources/StandardMacros.Can Execute Cosmetic Events`
    (:`True`
      (bind _statscomp (`/Game/MMOKit/MMO_Logic/Blueprints/Stats/BPI_Stats.GetStatsComponent`))
      (bind _creaturename (`/Game/MMOKit/MMO_Logic/Blueprints/Stats/BP_BaseStatsComponent.GetName` _statscomp))
      (`/Engine/EditorBlueprintResources/StandardMacros.IsValid` _returnvalue
        (:`Is Valid`
          (bind _eventbus (message `/Game/MMOKit/MMO_Logic/Blueprints/Interfaces/BPI_PlayerController.GetPlayerControllerEventBus` _returnvalue))
          (`/Game/MMOKit/MMO_Logic/Blueprints/EventBuses/BP_PlayerControllerEventBus.OnChannelMessage` _eventbus (`KismetMathLibrary.Conv_ByteToInt` (enumliteral `/Game/MMOKit/MMO_Logic/Blueprints/Enums/EChatMsgChannel` "NewEnumerator0")) (`KismetTextLibrary.Conv_TextToString` _creaturename) Message))))))

(event `/Game/MMOKit/MMO_Logic/Blueprints/Interfaces/BPI_Character.EmitUpdateReaction`
  (`self.UpdateReaction`))

(event `/Game/MMOKit/MMO_Logic/Blueprints/Interfaces/BPI_Reaction.SetLocalReaction`
  (params (NewReaction :type "/Game/MMOKit/MMO_Logic/Blueprints/Enums/EReaction Enum" :default "NewEnumerator0"))
  (set `self.Reaction` NewReaction)
  (`self.UpdateReaction`))

(fn `EmptyGear`
  (returns (Ok :type Boolean))
  (`/Game/MMOKit/MMO_Logic/Blueprints/BPFL_Lib.DestroyComponentIfValid` (`self.RhandMeshComponent`))
  (return false))

(fn `GetBattleStance`
  (returns (Stance :type "/Game/MMOKit/MMO_Logic/Blueprints/Enums/EBattleStance Enum"))
  (return (`/Game/MMOKit/MMO_Logic/Blueprints/BP_AppearanceComponent.GetBattleStance` (`self.AppearanceComponent`))))

(fn `GetCharacterEventBus`
  (returns (CharacterEventBus :type "/Game/MMOKit/MMO_Logic/Blueprints/EventBuses/BP_CharacterEventBus Object Reference"))
  ;[1 1 1] overwrite in child classes
  (return null))

(fn `GetDeathMontage`
  (returns (Montage :type "AnimMontage Object Reference"))
  ;[1 0.312 0.302] Get Death Montage
  (bind _full (`self.GetFullAppearance`))
  (return (`/Game/MMOKit/MMO_Logic/Blueprints/DataAssetTypes/CreatureAppearance.DeathMontage` (`.Appearance_2_26E153A448ABAAF3D63E13BDBF8DF3E1` (break `/Game/MMOKit/MMO_Logic/Blueprints/Struct/FAppearanceFull` _full)))))

(fn `GetFullAppearance`
  (returns (Full :type "/Game/MMOKit/MMO_Logic/Blueprints/Struct/FAppearanceFull Structure"))
  (return (`/Game/MMOKit/MMO_Logic/Blueprints/BP_AppearanceComponent.FullAppearance` (`self.AppearanceComponent`))))

(fn `GetInCombat`
  (returns (InCombat :type Boolean))
  (return (`self.InCombat`)))

(fn `GetMaxMoveSpeed`
  (returns (MaxSpeed :type "Float (double-precision)"))
  (return (`self.MaxMoveSpeed`)))

(fn `GetMeleeAttackOrigin`
  (returns (Origin :type "Transform Structure"))
  (return (`SceneComponent.K2_GetComponentToWorld` (`self.MeleeAttackVector`))))

(fn `GetPartialAppearance`
  (returns (PartialAppearance :type "/Game/MMOKit/MMO_Logic/Blueprints/Struct/FAppearancePartial Structure"))
  (bind ((`Sex_5_29930ADA4C0D945B21BBCC8DC49D7B50` _sex) (`Race_18_E6C95A3242408A8F95E330B7E9039D86` _race)) (break `/Game/MMOKit/MMO_Logic/Blueprints/Struct/FAppearanceFull` (`|GetArrayItem` (`/Game/MMOKit/MMO_Logic/Blueprints/BP_AppearanceComponent.AppearancesStack` (`self.AppearanceComponent`)))))
  (return (make `/Game/MMOKit/MMO_Logic/Blueprints/Struct/FAppearancePartial` _sex _race)))

(fn `GetReaction`
  (returns (Reaction :type "/Game/MMOKit/MMO_Logic/Blueprints/Enums/EReaction Enum"))
  (return "NewEnumerator1"))

(fn `GetSelectionDecal`
  (returns (Decal :type "DecalComponent Object Reference"))
  (return (`self.SelectionDecal`)))

(fn `GetStatsComponent`
  (returns (StatsComp :type "/Game/MMOKit/MMO_Logic/Blueprints/Stats/BP_BaseStatsComponent Object Reference"))
  ;[1 1 1] Override in child classes
  (return null))

(fn `GetTarget`
  (returns (TargetCharacter :type "Character Object Reference"))
  (return null))

(fn `IsAbilityOnCooldown`
  (params (Ability :type "/Game/MMOKit/MMO_Logic/Blueprints/DataAssetTypes/AbilityAsset Object Reference"))
  (returns (OnCooldown :type Boolean))
  (return (`/Game/MMOKit/MMO_Logic/Blueprints/BP_AbilitySystemComponent.IsAbilityOnCooldown` (`self.AbilitySystemComponent`) Ability)))

(fn `IsAlive`
  (returns (Alive :type Boolean))
  (bind _statscomp (`/Game/MMOKit/MMO_Logic/Blueprints/Stats/BPI_Stats.GetStatsComponent`))
  (`/Engine/EditorBlueprintResources/StandardMacros.IsValid` _statscomp
    (:`Is Valid`
      (return (`/Game/MMOKit/MMO_Logic/Blueprints/Stats/BP_BaseStatsComponent.IsAlive` _statscomp)))
    (:`Is Not Valid`
      (return false))))

(fn `IsOnGlobalCooldown`
  (returns (OnCooldown :type Boolean))
  (return (not (`/Game/MMOKit/MMO_Logic/Blueprints/BP_AbilitySystemComponent.DidGlobalCooldownEnd` (`self.AbilitySystemComponent`)))))

(fn `IsPlayerCharacter`
  (returns (IsPlayer :type Boolean))
  (return false))

(fn `OnRep_IsDead`
  (bind _mesh (`self.Mesh`))
  ;[1 0.312 0.302] IsDead notify is used to turn on/off ragdoll
  (bind _isplayer (`/Game/MMOKit/MMO_Logic/Blueprints/Interfaces/BPI_Character.IsPlayerCharacter`))
  (`PrimitiveComponent.SetCollisionProfileName` (`self.CapsuleComponent`) (select `bool` (`self.IsDead`) :`false` (select `bool` _isplayer :`false` "Pawn" :`true` "PawnPlayer" :!type "Name") :`true` "PawnDead") true)
  (`/Engine/EditorBlueprintResources/StandardMacros.Can Execute Cosmetic Events`
    (:`True`
      (if (`self.IsDead`)
        (set `self.CachedMeshRelativeTransform` (`SceneComponent.GetRelativeTransform` (`self.Mesh`)))
        (`PrimitiveComponent.SetCollisionProfileName` _mesh "Ragdoll" true)
        (`SkeletalMeshComponent.SetAllBodiesSimulatePhysics` _mesh true)
        (`SceneComponent.K2_DetachFromComponent` _mesh "KeepRelative" "KeepRelative" "KeepRelative" true)
        (else
          (`PrimitiveComponent.SetCollisionProfileName` _mesh "CharacterMesh" true)
          (`SkeletalMeshComponent.SetAllBodiesSimulatePhysics` _mesh false)
          (`SceneComponent.K2_AttachToComponent` _mesh (`self.CapsuleComponent`) "None" "SnapToTarget" "SnapToTarget" "SnapToTarget" false)
          (`SceneComponent.K2_SetRelativeTransform` _mesh (`self.CachedMeshRelativeTransform`) false true))))))

(fn `OnRep_Reaction`
  (`/Engine/EditorBlueprintResources/StandardMacros.Can Execute Cosmetic Events`
    (:`True`
      (`self.UpdateReaction`))))

(fn `RaycastMeleeAttack`
  (params (FromWhere :type "Transform Structure") (Reach :type "Float (double-precision)") (RaycastWidth :type "Float (double-precision)"))
  (returns (StatsComponent :type "/Game/MMOKit/MMO_Logic/Blueprints/Stats/BP_BaseStatsComponent Object Reference"))
  (locals (HitActor :type "Actor Object Reference") (HitActorReaction :type "/Game/MMOKit/MMO_Logic/Blueprints/Enums/EReaction Enum" :default "NewEnumerator0"))
  (bind _location (.location FromWhere))
  (bind _hitactorreaction (`local.HitActorReaction`))
  (bind (_outhit _returnvalue) (`KismetSystemLibrary.SphereTraceSingleForObjects` _location (+ _location (* (`KismetMathLibrary.GetForwardVector` (.rotation FromWhere)) Reach)) RaycastWidth (`|MakeArray` "ObjectTypeQuery3" :!type "EObjectTypeQuery Enum") true (`|MakeArray` self :!type "Actor Object Reference") "ForDuration" true (struct :`R` 1.0 :`A` 1.0) (struct :`G` 1.0 :`A` 1.0) 0.5))
  (if _returnvalue
    (bind _output_get (set `local.HitActor` (`.HitActor` (`GameplayStatics.BreakHitResult` _outhit))))
    (bind _isplayer (message `/Game/MMOKit/MMO_Logic/Blueprints/Interfaces/BPI_Character.IsPlayerCharacter` _output_get))
    (if _isplayer
      ;[1 1 1] if friendly reaction, return nothing
      (bind _reaction (message `/Game/MMOKit/MMO_Logic/Blueprints/Interfaces/BPI_Reaction.GetReaction` (`local.HitActor`)))
      (set `local.HitActorReaction` _reaction)
      (else
        (bind _reaction_2 (message `/Game/MMOKit/MMO_Logic/Blueprints/Interfaces/BPI_MobSpecific.GetMobInitialReaction` (`local.HitActor`)))
        (set `local.HitActorReaction` _reaction_2)))
    (if (or (`|EnumEquality` _hitactorreaction "NewEnumerator3") (`|EnumEquality` _hitactorreaction "NewEnumerator0"))
      (return null)
      (else
        (bind _statscomp (message `/Game/MMOKit/MMO_Logic/Blueprints/Stats/BPI_Stats.GetStatsComponent` (`local.HitActor`)))
        (return _statscomp)))))

(fn `SetBody`
  (params (NewMesh :type "SkeletalMesh Object Reference") (AnimBp :type "AnimInstance Class Reference") (Sex :type "/Game/MMOKit/MMO_Logic/Blueprints/Enums/ECreatureSex Enum" :default "NewEnumerator0") (CreRace :type "/Game/MMOKit/MMO_Logic/Blueprints/Enums/ECreatureRace Enum" :default "NewEnumerator2"))
  (returns (Changed :type Boolean))
  (locals (ChangedMesh :type Boolean))
  (bind _mesh (`self.Mesh`))
  (`MmoUtilities.LogString` (`KismetStringLibrary.Concat_StrStr` "Set body:" (`KismetSystemLibrary.GetDisplayName` NewMesh)))
  (`|ExecutionSequence`
    (:`then_0`
      (bind _output_get (set `local.ChangedMesh` (or (!= (`SkeletalMeshComponent.GetSkeletalMeshAsset` (`self.Mesh`)) (`local.NewMesh`)) (!= (`SkeletalMeshComponent.AnimClass` (`self.Mesh`)) (`local.AnimBp`)))))
      (if _output_get
        (`SkeletalMeshComponent.SetAnimInstanceClass` _mesh null)
        (`SkinnedMeshComponent.SetSkinnedAssetAndUpdate` _mesh (`local.NewMesh`) false)
        (`SkeletalMeshComponent.SetAnimInstanceClass` _mesh (`local.AnimBp`))
        (`/Game/MMOKit/MMO_Logic/Blueprints/BPFL_Lib.DestroyComponentIfValid` (`self.LeftEyeComponent`))
        (`/Game/MMOKit/MMO_Logic/Blueprints/BPFL_Lib.DestroyComponentIfValid` (`self.RightEyeComponent`))
        (else
          (return (`local.ChangedMesh`)))))
    (:`then_1`
      (`/Engine/EditorBlueprintResources/StandardMacros.Can Execute Cosmetic Events`
        (:`True`
          (bind _should (`self.ShouldAttachEyes`))
          (if _should
            (`|ExecutionSequence`
              (:`then_0`
                (bind _returnvalue (`|AddComponentByClass` "/Script/Engine.StaticMeshComponent" true))
                (`PrimitiveComponent.SetCollisionEnabled` _returnvalue "NoCollision")
                (`SceneComponent.K2_AttachToComponent` _returnvalue (`self.Mesh`) "eye_l" "KeepRelative" "KeepRelative" "KeepRelative" true)
                (`StaticMeshComponent.SetStaticMesh` _returnvalue "/Game/MMOKit/MMO_Assets/Eye/SM_Eye.SM_Eye")
                (`PrimitiveComponent.SetMaterial` _returnvalue 0 (select `/Game/MMOKit/MMO_Logic/Blueprints/Enums/ECreatureSex` (`local.Sex`) :`NewEnumerator0` "/Game/MMOKit/MMO_Assets/Eye/MI_EyeRefractive_Man.MI_EyeRefractive_Man" :`NewEnumerator1` "/Game/MMOKit/MMO_Assets/Eye/MI_EyeRefractive_Girl.MI_EyeRefractive_Girl" :!type "MaterialInterface Object Reference"))
                (set `self.LeftEyeComponent` _returnvalue)
                (`SceneComponent.SetVisibility` _returnvalue (`SceneComponent.bVisible` (`self.Mesh`)) false))
              (:`then_1`
                (bind _returnvalue_2 (`|AddComponentByClass` "/Script/Engine.StaticMeshComponent" true))
                (`PrimitiveComponent.SetCollisionEnabled` _returnvalue_2 "NoCollision")
                (`SceneComponent.K2_AttachToComponent` _returnvalue_2 (`self.Mesh`) "eye_r" "KeepRelative" "KeepRelative" "KeepRelative" true)
                (`StaticMeshComponent.SetStaticMesh` _returnvalue_2 "/Game/MMOKit/MMO_Assets/Eye/SM_Eye.SM_Eye")
                (`PrimitiveComponent.SetMaterial` _returnvalue_2 0 (select `/Game/MMOKit/MMO_Logic/Blueprints/Enums/ECreatureSex` (`local.Sex`) :`NewEnumerator0` "/Game/MMOKit/MMO_Assets/Eye/MI_EyeRefractive_Man.MI_EyeRefractive_Man" :`NewEnumerator1` "/Game/MMOKit/MMO_Assets/Eye/MI_EyeRefractive_Girl.MI_EyeRefractive_Girl" :!type "MaterialInterface Object Reference"))
                (set `self.RightEyeComponent` _returnvalue_2)
                (`SceneComponent.SetVisibility` _returnvalue_2 (`SceneComponent.bVisible` (`self.Mesh`)) false)))))))
    (:`then_2`
      (return (`local.ChangedMesh`)))))

(fn `ShouldAttachEyes`
  (returns (Should :type Boolean))
  (return (`/Game/MMOKit/MMO_Logic/Blueprints/BP_AppearanceComponent.ShouldAttachEyes` (`self.AppearanceComponent`))))

(fn `UserConstructionScript`)