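; WoW-style MMO camera component, derived from a base camera component, that sets up the owner's boom, cursor and rotation rules.
; RMB makes the character follow controller yaw and turns A/D into strafing; otherwise A/D rotates the character, carrying the camera unless LMB is held.
; Jogging without look input gradually pulls the camera behind the character.
; Zoom input sets a clamped arm length eased on Tick; rotation changes are sent to the server.
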(event `self.ChatLostFocus`
  (bind _ownercontroller (`self.OwnerController`))
  ;[1 1 1] Chat Lost Focus
  (`WidgetBlueprintLibrary.SetInputMode_GameOnly` _ownercontroller)
  (`WidgetBlueprintLibrary.SetInputMode_GameAndUIEx` _ownercontroller null)
  (set `PlayerController.bShowMouseCursor` true _ownercontroller))

(event `self.ReceiveBeginPlay`
  (bind _ownercharacter (`self.OwnerCharacter`))
  (bind _ownercontroller (`self.OwnerController`))
  (bind _followcamera (`/Game/MMOKit/MMO_Logic/Blueprints/BP_PlayerCharacter.FollowCamera` (`self.OwnerCharacter`)))
  (bind _cameraboom (`/Game/MMOKit/MMO_Logic/Blueprints/BP_PlayerCharacter.CameraBoom` (`self.OwnerCharacter`)))
  (bind _charactermovement (`Character.CharacterMovement` _ownercharacter))
  ;[1 1 1] BeginPlay: initialize camera and some variables
  (`parent.ReceiveBeginPlay`)
  (bind _output_get (set `SpringArmComponent.TargetArmLength` 400.0 _cameraboom))
  (set `self.ZoomTo` _output_get)
  (`SceneComponent.K2_SetRelativeLocation` _cameraboom (0.0 0.0 75.0) false false)
  (`SceneComponent.K2_SetRelativeLocation` _followcamera (0.0 0.0 0.0) false false)
  (`SceneComponent.SetRelativeScale3D` _followcamera (1.0 1.0 1.0))
  (`WidgetBlueprintLibrary.SetInputMode_GameAndUIEx` _ownercontroller null "LockOnCapture")
  (set `PlayerController.bShowMouseCursor` true _ownercontroller)
  (set `Pawn.bUseControllerRotationYaw` false _ownercharacter)
  (set `CharacterMovementComponent.RotationRate` (struct :`Yaw` 500.0) _charactermovement) ; just resetting it to default, not that we use it in thos camera mode
  (bind _output_get_2 (set `CharacterMovementComponent.bUseControllerDesiredRotation` false _charactermovement))
  (`/Game/MMOKit/MMO_Logic/Blueprints/BP_PlayerCharacter.SetUseControllerRotationOnServer` (`self.OwnerCharacter`) _output_get_2)
  (set `CharacterMovementComponent.RotationRate` (`KismetMathLibrary.MakeRotator` 0.0 0.0 -1.0) (`Character.CharacterMovement` (`self.OwnerCharacter`)))
  (`/Game/MMOKit/MMO_Logic/Blueprints/BP_PlayerCharacter.SetRotationRateOnServer` (`self.OwnerCharacter`) -1.0)
  (`SceneComponent.SetVisibility` (`Character.Mesh` (`self.OwnerCharacter`)) true true))

(event `self.OnRMB`
  (params (Down :type Boolean))
  ;[1 1 1] Whenever RMB is pressed down, force the Character follow the Controller's rotation
  (bind _output_get (set `Pawn.bUseControllerRotationYaw` Down (`self.OwnerCharacter`)))
  (`/Game/MMOKit/MMO_Logic/Blueprints/BP_PlayerCharacter.SetUseControllerRotationOnServer` (`self.OwnerCharacter`) _output_get))

(event `self.Jog`
  (params (InputVector :type "Vector2D Structure"))
  (bind (_x _y) (`KismetMathLibrary.BreakVector2D` InputVector))
  (bind _ownercontroller (`self.OwnerController`))
  (bind _ownercontroller_2 (`self.OwnerController`))
  (bind _yaw (.yaw (`Controller.GetControlRotation` (`self.OwnerController`))))
  (bind _returnvalue (`KismetMathLibrary.MakeRotator` 0.0 0.0 (.yaw (`Actor.K2_GetActorRotation` (`self.OwnerCharacter`)))))
  (bind _returnvalue_2 (`KismetMathLibrary.NormalizeAxis` (- (`KismetMathLibrary.NormalizeAxis` (.yaw (`Actor.K2_GetActorRotation` (`self.OwnerCharacter`)))) (`KismetMathLibrary.NormalizeAxis` (.yaw (`Controller.GetControlRotation` (`self.OwnerController`)))))))
  ;[1 1 1] Jog in the direction of the Player Character
  (`PawnMovementComponent.AddInputVector` (`Character.CharacterMovement` (`self.OwnerCharacter`)) (+ (* (`KismetMathLibrary.GetForwardVector` _returnvalue) _y) (* (`KismetMathLibrary.GetRightVector` _returnvalue) _x)) false)
  ;[1 1 1] If we're jogging, LMB & RMB are not pressed, and the camera is not set straight, slowly pull it straight as we jog
  (if (and (`KismetMathLibrary.IsZero2D` (`/Game/MMOKit/MMO_Logic/Blueprints/BP_PlayerController.GetIA_LookAround` _ownercontroller_2)) (not (`/Game/MMOKit/MMO_Logic/Blueprints/BP_PlayerController.IsLmbDown` _ownercontroller)) (not (`/Game/MMOKit/MMO_Logic/Blueprints/BP_PlayerController.IsRmbDown` _ownercontroller)) (not (`Pawn.bUseControllerRotationYaw` (`self.OwnerCharacter`))) (!= (.yaw (`Controller.GetControlRotation` (`self.OwnerController`))) (.yaw (`Actor.K2_GetActorRotation` (`self.OwnerCharacter`)))) (== (`/Game/MMOKit/MMO_Logic/Blueprints/BP_PlayerController.GetIa_TurnAround` _ownercontroller_2) 0.0))
    ;[1 1 1] This is a simple math formula to pull the camera towards a straight position on each tick while jogging.
    ; Our target angle is: Character's Yaw
    ; Our current angle is: Controller's Yaw
    ; The difference between them is = Normalize(Character's Yaw) - Normalize(Controller's Yaw)
    ; Then normalize the difference itself and check its sign.
    ; If it's a plus sign, just add a bit of degrees (currently 150 * deltaTime) to Controller's yaw.
    ; If it's a negative sign, substract the same amount.
    ; If the difference is negligible (<= 3 degrees), then just set it to exactly Controller's Yaw already.
    (`Controller.SetControlRotation` (`self.OwnerController`) (`KismetMathLibrary.MakeRotator` (.roll (`Controller.GetControlRotation` (`self.OwnerController`))) (.pitch (`Controller.GetControlRotation` (`self.OwnerController`))) (`KismetMathLibrary.SelectFloat` (+ _yaw (* (`GameplayStatics.GetWorldDeltaSeconds`) (`KismetMathLibrary.SignOfFloat` _returnvalue_2) 150.0)) _yaw (> (`KismetMathLibrary.Abs` _returnvalue_2) 3.0))))))

(event `self.LookAround`
  (params (InputVector :type "Vector2D Structure"))
  (bind (_x _y) (`KismetMathLibrary.BreakVector2D` InputVector))
  (bind _turnratemousegamepad (`/Game/MMOKit/MMO_Logic/Blueprints/BP_PlayerController.TurnRateMouseGamepad` (`self.OwnerController`)))
  ;[1 1 1] LookAround
  ;;[1 1 1 0] (If looking around with RMB, the Character will turn too, see OnRMB Event)
  ;; Note: gamepad and mouse are polled differently in UE5.  For some reason, the mouse is FPS agnostic,
  ;; while the gamepad requires deltaTime. In this case, I've not fixed the gamepad, because:
  ;; a) this may get fixed in UE5 eventually
  ;; b) most MMO clients don't go beyond 60 fps
  ;; c) most MMOs aren't relient on gamepads
  ;; If you want to fix this, you have to decouple LookAround into two InputActions: MouseLookAround and GamepadLookAround.
  (`PlayerController.AddYawInput` (`self.OwnerController`) (* _turnratemousegamepad _x))
  (`PlayerController.AddPitchInput` (`self.OwnerController`) (* _turnratemousegamepad _y)))

(event `self.ZoomInOut`
  (params (X :type "Float (double-precision)"))
  ;[1 1 1] Zoom In/Out is executed in the Tick event
  (set `self.ZoomAlpha` (`KismetMathLibrary.SelectFloat` 0.2 (`KismetMathLibrary.SelectFloat` (`self.ZoomAlpha`) 0.0 (< (`self.ZoomAlpha`) 0.2)) (`KismetMathLibrary.InRange_FloatFloat` (`self.ZoomAlpha`) 0.2 1.0 false false)))
  (set `self.ZoomFrom` (`SpringArmComponent.TargetArmLength` (`/Game/MMOKit/MMO_Logic/Blueprints/BP_PlayerCharacter.CameraBoom` (`self.OwnerCharacter`))))
  (set `self.ZoomTo` (`KismetMathLibrary.FClamp` (+ (* X 100.0) (`self.ZoomTo`)) 100.0 1200.0)))

(event `ZoomUpdate`
  ;[1 1 1] Zoom In/Out is executed in the Tick event
  (if (< (`self.ZoomAlpha`) 1.0)
    (set `SpringArmComponent.TargetArmLength` (`|EaseFunction` "EaseInOut" (`self.ZoomAlpha`) (`self.ZoomFrom`) (`self.ZoomTo`)) (`/Game/MMOKit/MMO_Logic/Blueprints/BP_PlayerCharacter.CameraBoom` (`self.OwnerCharacter`)))
    (set `self.ZoomAlpha` (+ (`self.ZoomAlpha`) (`KismetMathLibrary.SafeDivide` (`GameplayStatics.GetWorldDeltaSeconds`) 0.3))) ; Increase alpha on each tick by\nDeltaTime*(1/ZoomTime)\n1/ZoomTime is ZoomSpeed
  ))

(event `self.TurnAround`
  (params (X :type "Float (double-precision)"))
  (bind _ownercharacter (`self.OwnerCharacter`))
  (bind _ownercontroller (`self.OwnerController`))
  (bind _returnvalue (`KismetMathLibrary.MakeRotator` (.roll (`Actor.K2_GetActorRotation` (`self.OwnerCharacter`))) (.pitch (`Actor.K2_GetActorRotation` (`self.OwnerCharacter`))) (+ (.yaw (`Actor.K2_GetActorRotation` (`self.OwnerCharacter`))) (* (`KismetMathLibrary.FClamp` (`GameplayStatics.GetWorldDeltaSeconds`) 0.016667 5.0) (`self.TurnSpeed`) X))))
  ;[1 1 1] Turn Around (using A/D): the camera follows, unless LMB is pressed
  (if (not (`/Game/MMOKit/MMO_Logic/Blueprints/BP_PlayerController.IsRmbDown` (`self.OwnerController`)))
    (`Actor.K2_SetActorRotation` _ownercharacter _returnvalue false)
    (`/Game/MMOKit/MMO_Logic/Blueprints/BP_PlayerCharacter.SetActorRotationOnServer` _ownercharacter _returnvalue)
    (if (not (`/Game/MMOKit/MMO_Logic/Blueprints/BP_PlayerController.IsLmbDown` (`self.OwnerController`)))
      (`Controller.SetControlRotation` _ownercontroller (`KismetMathLibrary.MakeRotator` (.roll (`Controller.GetControlRotation` _ownercontroller)) (.pitch (`Controller.GetControlRotation` _ownercontroller)) (+ (.yaw (`Controller.GetControlRotation` _ownercontroller)) (* (`GameplayStatics.GetWorldDeltaSeconds`) (`self.TurnSpeed`) X)))))
    (else
      ;[1 1 1] TurnAround + RMB is Strafe
      (`self.Jog` (`KismetMathLibrary.MakeVector2D` X)))))

(event `self.ReceiveTick`
  (params (DeltaSeconds :type "Float (single-precision)"))
  ;[1 1 1] Tick
  (`self.ZoomUpdate`))