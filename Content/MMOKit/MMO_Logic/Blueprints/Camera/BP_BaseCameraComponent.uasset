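; Base camera component for player characters, meant to be subclassed per camera style and added at runtime or in editor.
; On BeginPlay it binds player controller input to overridable handlers where cosmetic events can run, and death/resurrection events from the controller's message bus, retrying each tick until available.
; Handlers are empty except Jump, which makes the character jump.
; GetCameraAttackOrigin is a stub for child cameras to supply targetless combat spherecast origins.
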(event `self.ReceiveBeginPlay`
  ;[1 1 1] The children of this component can be added to a Character at runtime or in Editor
  (`|ExecutionSequence`
    (:`then_0`
      (bind _asbp_player_character (cast `/Game/MMOKit/MMO_Logic/Blueprints/BP_PlayerCharacter` (`self.GetOwner`)))
      (set `self.OwnerCharacter` _asbp_player_character)
      (`/Engine/EditorBlueprintResources/StandardMacros.Can Execute Cosmetic Events`
        (:`True`
          (bind _asbp_player_controller (cast `/Game/MMOKit/MMO_Logic/Blueprints/BP_PlayerController` (`Pawn.GetController` (`self.OwnerCharacter`)) :!label _label)
            (:`then`
              (set `self.OwnerController` _asbp_player_controller)
              (add `/Game/MMOKit/MMO_Logic/Blueprints/BP_PlayerController.OnJog` _asbp_player_controller (delegate `Jog`))
              (add `/Game/MMOKit/MMO_Logic/Blueprints/BP_PlayerController.OnJump` _asbp_player_controller (delegate `Jump`))
              (add `/Game/MMOKit/MMO_Logic/Blueprints/BP_PlayerController.OnRmbDown` _asbp_player_controller (delegate `OnRMB`))
              (add `/Game/MMOKit/MMO_Logic/Blueprints/BP_PlayerController.OnLmbDown` _asbp_player_controller (delegate `OnLMB`))
              (add `/Game/MMOKit/MMO_Logic/Blueprints/BP_PlayerController.OnLookAround` _asbp_player_controller (delegate `LookAround`))
              (add `/Game/MMOKit/MMO_Logic/Blueprints/BP_PlayerController.OnTurnAround` _asbp_player_controller (delegate `TurnAround`))
              (add `/Game/MMOKit/MMO_Logic/Blueprints/BP_PlayerController.OnZoomInOut` _asbp_player_controller (delegate `ZoomInOut`))
              (add `/Game/MMOKit/MMO_Logic/Blueprints/BP_PlayerController.OnJogStart` _asbp_player_controller (delegate `JogStart`))
              (add `/Game/MMOKit/MMO_Logic/Blueprints/BP_PlayerController.OnJogEnd` _asbp_player_controller (delegate `JogEnd`))
              (add `/Game/MMOKit/MMO_Logic/Blueprints/BP_PlayerController.OnMenuModeToggle` _asbp_player_controller (delegate `MenuModeToggle`))
              (add `/Game/MMOKit/MMO_Logic/Blueprints/BP_PlayerController.OnChatLostFocus` _asbp_player_controller (delegate `ChatLostFocus`)))
            (:`CastFailed`
              (`KismetSystemLibrary.DelayUntilNextTick`) ; wait for PlayerController in case it's not initialized yet
              (goto _label))))))
    (:`then_1`
      (bind _eventbus (message `/Game/MMOKit/MMO_Logic/Blueprints/Interfaces/BPI_PlayerController.GetPlayerControllerEventBus` (`GameplayStatics.GetPlayerController` 0) :!label _label_2))
      (`/Engine/EditorBlueprintResources/StandardMacros.IsValid` _eventbus
        (:`Is Valid`
          (add `/Game/MMOKit/MMO_Logic/Blueprints/EventBuses/BP_PlayerControllerEventBus.OnCharacterDied` _eventbus (delegate `OnCharacterDied`))
          (add `/Game/MMOKit/MMO_Logic/Blueprints/EventBuses/BP_PlayerControllerEventBus.OnCharacterResurrected` _eventbus (delegate `OnCharacterResurrected`)))
        (:`Is Not Valid`
          (`KismetSystemLibrary.DelayUntilNextTick`)
          (`MmoUtilities.LogString` "CameraComponent: Delay by 1 tick")
          (goto _label_2))))))

(event `Jog`
  (params (InputVector :type "Vector2D Structure"))
  ;[1 1 1] These events can be overridden in child classes
)

(event `Jump`
  ;[1 1 1] These events can be overridden in child classes
  (`Character.Jump` (`self.OwnerCharacter`)))

(event `OnRMB`
  (params (Down :type Boolean))
  ;[1 1 1] These events can be overridden in child classes
)

(event `OnLMB`
  (params (Down :type Boolean))
  ;[1 1 1] These events can be overridden in child classes
)

(event `LookAround`
  (params (InputVector :type "Vector2D Structure"))
  ;[1 1 1] These events can be overridden in child classes
)

(event `TurnAround`
  (params (X :type "Float (double-precision)"))
  ;[1 1 1] These events can be overridden in child classes
)

(event `ZoomInOut`
  (params (X :type "Float (double-precision)"))
  ;[1 1 1] These events can be overridden in child classes
)

(event `JogStart`
  ;[1 1 1] These events can be overridden in child classes
)

(event `JogEnd`
  ;[1 1 1] These events can be overridden in child classes
)

(event `MenuModeToggle`
  (params (On :type Boolean))
  ;[1 1 1] These events can be overridden in child classes
)

(event `ChatLostFocus`
  ;[1 1 1] These events can be overridden in child classes
)

(event `OnCharacterDied`)

(event `OnCharacterResurrected`)

(fn `Get Camera Attack Origin`
  (returns (Origin :type "Transform Structure"))
  ;[1 1 1] To override in other cameras, but not needed for WoW type camera
  ; Returns the origin for a spherecast in targetless combat
  (return))