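; Base actor component for character stats that tracks replicated current and max HP, with damage, healing and resurrection.
; Damage and healing clamp HP and only affect living owners; death and resurrection send DieMessage or ResurrectMessage to the owning actor.
; DieFastOwner zeroes HP ahead of normal replication, and the RepNotifies broadcast HP updates.
; GetName and EmitNameUpdated are placeholders, the latter meant for child classes to override.
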(event `DieFastOwner`
  ;[1 0.312 0.302] Sets our character's HP faster than a normal replication would
  (set `self.CurHp` 0))

(event `TakeDamage`
  (params (Attacker :type "Character Object Reference") (Dmg :type Integer))
  ;[0.4452 0.6332 1] Take dmg (server)
  (if (`self.IsAlive`)
    (set `self.CurHp` (`KismetMathLibrary.Clamp` (- (`self.CurHp`) Dmg) 0 (`self.MaxHp`)))
    (if (not (`self.IsAlive`))
      (`self.DieFastOwner`)
      (message `/Game/MMOKit/MMO_Logic/Blueprints/Interfaces/BPI_Character.Die` (`self.GetOwner`) Attacker))))

(event `HealHp`
  (params (Healer :type "Character Object Reference") (HpHealed :type Integer))
  (if (`self.IsAlive`)
    (set `self.CurHp` (`KismetMathLibrary.Clamp` (+ (`self.CurHp`) HpHealed) 0 (`self.MaxHp`)))))

(event `Resurrect`
  ;[0.4452 0.6332 1] Resurrect
  (if (not (`self.IsAlive`))
    (set `self.CurHp` (`self.MaxHp`))
    (if (`self.IsAlive`)
      (message `/Game/MMOKit/MMO_Logic/Blueprints/Interfaces/BPI_Character.Resurrect` (`self.GetOwner`)))))

(event `EmitNameUpdated`)

(event `EmitHpUpdated`
  ;[1 0.312 0.302] Emit Hp Updated
  (`self.OnHpUpdated` (`self.CurHp`) (`self.MaxHp`)))

(fn `GetName`
  (returns (CreatureName :type Text))
  (return "NoName"))

(fn `IsAlive`
  (returns (Alive :type Boolean))
  (return (> (`self.CurHp`) 0)))

(fn `OnRep_CurHp`
  (`self.EmitHpUpdated`))

(fn `OnRep_MaxHp`
  (`self.EmitHpUpdated`))