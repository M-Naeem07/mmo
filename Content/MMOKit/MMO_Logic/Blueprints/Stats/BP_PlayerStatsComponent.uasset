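; Player stats component for the MMO kit, extending a parent stats component with character name, class, resurrection requests and health regeneration.
; Timers start regen at play where cosmetic events are not executed, pause it for seven seconds after damage, then heal a percentage of max HP periodically until full.
; Name replication fires an update event.
; Initialize and GetSerializedStats load and export name, HP and class through a player stats struct.
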(event `self.ReceiveBeginPlay`
  (`parent.ReceiveBeginPlay`)
  (`/Engine/EditorBlueprintResources/StandardMacros.Can Execute Cosmetic Events`
    (:`False`
      ;[0.4452 0.6332 1] start health regen on entry
      (`self.StartRegen`))))

(event `RequestResurrect`
  ;[0.4452 0.6332 1] Player requests resurrect
  (if (not (`self.IsAlive`))
    (`self.Resurrect`)))

(event `self.TakeDamage`
  (params (Attacker :type "Character Object Reference") (Dmg :type Integer))
  ;[0.4452 0.6332 1] health regen starts 7 secs after taking no damage
  (`parent.TakeDamage` Attacker Dmg)
  (`KismetSystemLibrary.K2_ClearAndInvalidateTimerHandle` (`self.RegenTickTimer`))
  (bind _returnvalue (`KismetSystemLibrary.K2_SetTimerDelegate` (delegate `StartRegen`) 7.0))
  (set `self.RegenStartTimer` _returnvalue))

(event `StartRegen`
  ;[0.4452 0.6332 1] health regen starts 7 secs after taking no damage
  (bind _returnvalue (`KismetSystemLibrary.K2_SetTimerDelegate` (delegate `RegenTick`) 2.0 true))
  (set `self.RegenTickTimer` _returnvalue))

(event `self.EmitNameUpdated`
  (`self.OnNameUpdated` (`self.PlayerName`)))

(event `RegenTick`
  ;[0.4452 0.6332 1] health regen starts 7 secs after taking no damage
  (if (and (`self.IsAlive`) (< (`self.CurHp`) (`self.MaxHp`)))
    (`self.HealHp` null (`KismetMathLibrary.FTrunc` (* (`KismetMathLibrary.Conv_IntToDouble` (`self.MaxHp`)) 0.03)))
    (if (== (`self.CurHp`) (`self.MaxHp`))
      (`KismetSystemLibrary.K2_ClearAndInvalidateTimerHandle` (`self.RegenTickTimer`)))))

(event `/Game/MMOKit/MMO_Logic/Blueprints/Interfaces/BPI_PlayerStats.SetName`
  (params (NewName :type String))
  (set `self.PlayerName` NewName))

(event `/Game/MMOKit/MMO_Logic/Blueprints/Interfaces/BPI_PlayerStats.SetClass`
  (params (NewClass :type "/Game/MMOKit/MMO_Logic/Blueprints/Enums/EClassType Enum" :default "NewEnumerator0"))
  (set `self.RpgClass` NewClass))

(fn `GetClass`
  (returns (RpgClass :type "/Game/MMOKit/MMO_Logic/Blueprints/Enums/EClassType Enum"))
  (return (`self.RpgClass`)))

(fn `GetName`
  (returns (CreatureName :type Text))
  (return (`KismetTextLibrary.Conv_StringToText` (`self.PlayerName`))))

(fn `GetSerializedStats`
  (returns (StatsStruct :type "/Game/MMOKit/MMO_Logic/Blueprints/Struct/FStatsPlayer Structure"))
  (locals (JsonObj :type "JsonObjectWrapper Structure"))
  (return (make `/Game/MMOKit/MMO_Logic/Blueprints/Struct/FStatsPlayer` (`self.PlayerName`) (`self.CurHp`) (`self.MaxHp`) (`self.RpgClass`))))

(fn `Initialize`
  (params (InStats :type "/Game/MMOKit/MMO_Logic/Blueprints/Struct/FStatsPlayer Structure"))
  (bind (_charname _curhp _maxhp _rpgclass) (break `/Game/MMOKit/MMO_Logic/Blueprints/Struct/FStatsPlayer` InStats))
  (`|ExecutionSequence`
    (:`then_0`
      (set `self.PlayerName` _charname)
      (set `self.MaxHp` _maxhp)
      (set `self.CurHp` (`KismetMathLibrary.Max` _curhp 1))
      (set `self.RpgClass` _rpgclass))
    (:`then_1`
      (if (`self.IsAlive`)
        _))))

(fn `OnRep_GuildName`)

(fn `OnRep_PlayerName`
  (`self.EmitNameUpdated`))