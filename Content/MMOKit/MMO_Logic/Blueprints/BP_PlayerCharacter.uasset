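; Player character for an MMO kit, handling interaction, aggro, appearance updates, death and graveyard resurrection.
; On the local client it waits for the controller's event bus, then swaps in camera and interaction components matching the camera type (first-person, over-shoulder or WoW-style).
; Construction adds an event bus, plus stats and an aggro sphere when cosmetics are off.
; Interaction and rotation relay to the server; death and resurrection notify the controller's event bus.
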(event `OnMenuVignette`
  (params (On :type Boolean))
  ;[1 0.312 0.302] Vignette effect on Menu Mode on/off
  (set `CameraComponent.PostProcessSettings` (select `bool` On :`false` (make `PostProcessSettings`) :`true` (make `PostProcessSettings` :`VignetteIntensity` 0.8)) (`self.FollowCamera`)))

(event `self.SetNameplateWidget`
  ;[1 0.312 0.302] Set NamePlate Widget
  (`self.IsOurCharacter`
    (:`No`
      (bind _returnvalue (`|CreateWidget` "/Game/MMOKit/MMO_Logic/Widgets/WBP_PlayerNameplate.WBP_PlayerNameplate_C" null self))
      (`WidgetComponent.SetWidget` (`self.NameplateWidget`) _returnvalue))))

(event `StopInteractOnServer`
  (params (Interactable :type "/Game/MMOKit/MMO_Logic/Blueprints/Interaction/BPI_Interactable Interface"))
  ;[0.4452 0.6332 1] Interact on Server
  (`/Engine/EditorBlueprintResources/StandardMacros.IsValid` (`KismetSystemLibrary.Conv_InterfaceToObject` Interactable)
    (:`Is Valid`
      (`/Game/MMOKit/MMO_Logic/Blueprints/Interaction/BPI_Interactable.StopInteract` Interactable self))))

(event `SignUpToEvents`
  ;[1 0.312 0.302] Sign up to events
  (`/Engine/EditorBlueprintResources/StandardMacros.Can Execute Cosmetic Events`
    (:`True`
      (add `/Game/MMOKit/MMO_Logic/Blueprints/BP_PlayerController.OnMenuModeToggle` (`self.GetBpController`) (delegate `OnMenuVignette`)))))

(event `ObserveInteractable`
  (params (Interactable :type "/Game/MMOKit/MMO_Logic/Blueprints/Interaction/BPI_Interactable Interface"))
  ;[1 0.312 0.302] Interact on Client
  (`/Game/MMOKit/MMO_Logic/Blueprints/Interaction/BP_InteractionSystemBase.StartObserveInteractable` (`self.InteractionSystemComponent`) Interactable) ; Will cause MenuToggle in 1/3 Person\nWill cause inventory to open in WoW\nWill open Loot Widget
)

(event `InteractOnServer`
  (params (Interactable :type "/Game/MMOKit/MMO_Logic/Blueprints/Interaction/BPI_Interactable Interface"))
  ;[0.4452 0.6332 1] Interact on Server
  (`/Game/MMOKit/MMO_Logic/Blueprints/Interaction/BPI_Interactable.Interact` Interactable self))

(event `StopInteractLocal`
  (params (Interactable :type "/Game/MMOKit/MMO_Logic/Blueprints/Interaction/BPI_Interactable Interface"))
  ;[1 0.312 0.302] Interact on Client
  (`self.StopInteractOnServer` Interactable)
  (`/Game/MMOKit/MMO_Logic/Blueprints/Interaction/BP_InteractionSystemBase.StopInteract` (`self.InteractionSystemComponent`) :!label _label) ; will interrupt observing interactable
)

(event `ReceiveLootClient`
  (params (Items :type "Array of PrimaryAssetId Structure") (Amounts :type "Array of Integer"))
  ;[1 0.312 0.302] Interact on Client
  (`/Game/MMOKit/MMO_Logic/Blueprints/Interaction/BP_InteractionSystemBase.LootReceived` (`self.InteractionSystemComponent`) Items Amounts))

(event `StopInteractClient`
  ;[1 0.312 0.302] Interact on Client
  (goto _label))

(event `self.ReceiveBeginPlay`
  ;[1 1 1] BeginPlay
  (`parent.ReceiveBeginPlay`)
  (`MmoUtilities.LogString` "Char: BeginPlay"))

(event `self.ReceiveTick`
  (params (DeltaSeconds :type "Float (single-precision)"))
  ;[1 1 1] BeginPlay
  (`parent.ReceiveTick` DeltaSeconds))

(event `AddAggroSphere`
  ;[0.4452 0.6332 1] Add aggro sphere (Server-only, from BeginPlay)
  (bind _returnvalue (`AddComponent|NODE_AddSphereComponent-1`))
  (set `self.AggroRangeSphereCollider` _returnvalue)
  (`SphereComponent.SetSphereRadius` (`self.AggroRangeSphereCollider`) 500.0 false)
  (`PrimitiveComponent.SetCollisionProfileName` (`self.AggroRangeSphereCollider`) "AggroSphere" true)
  (add `PrimitiveComponent.OnComponentBeginOverlap` (`self.AggroRangeSphereCollider`) (delegate `OnAggroSphereBeginOverlap`))
  (add `PrimitiveComponent.OnComponentEndOverlap` (`self.AggroRangeSphereCollider`) (delegate `OnAggroSphereEndOverlap`)))

(event `self.ReceiveRestarted`
  ;[1 1 1] BeginPlay
  (`MmoUtilities.LogString` "BeginPlay: Player Character Restarted")
  (`self.IsOurCharacter`
    (:`Yes`
      (bind _eventbus (message `/Game/MMOKit/MMO_Logic/Blueprints/Interfaces/BPI_PlayerController.GetPlayerControllerEventBus` (`GameplayStatics.GetPlayerController` 0) :!label _label_2))
      ;;[1 1 1] Wait for Controller, allow it to process BeginPlay
      (`/Engine/EditorBlueprintResources/StandardMacros.IsValid` _eventbus
        (:`Is Valid`
          (`KismetSystemLibrary.DelayUntilNextTick`)
          (`self.SignUpToEvents`)
          (`self.SetupComponents`)
          (set `self.ComponentsAreSetUp` true))
        (:`Is Not Valid`
          (`KismetSystemLibrary.DelayUntilNextTick`)
          (`MmoUtilities.LogString` "PlayerCharacter: Delay by 1 frame OnRestarted")
          (goto _label_2))))))

(event `OnAggroSphereBeginOverlap`
  (params (OverlappedComponent :type "PrimitiveComponent Object Reference") (OtherActor :type "Actor Object Reference") (OtherComp :type "PrimitiveComponent Object Reference") (OtherBodyIndex :type Integer) (bFromSweep :type Boolean) (SweepResult :type "HitResult Structure (by ref)"))
  ;[0.4452 0.6332 1] Add aggro sphere (Server-only, from BeginPlay)
  (message `/Game/MMOKit/MMO_Logic/Blueprints/Interfaces/BPI_MobSpecific.OnPlayerEnteredAggro` OtherActor self))

(event `OnAggroSphereEndOverlap`
  (params (OverlappedComponent :type "PrimitiveComponent Object Reference") (OtherActor :type "Actor Object Reference") (OtherComp :type "PrimitiveComponent Object Reference") (OtherBodyIndex :type Integer))
  ;[0.4452 0.6332 1] Add aggro sphere (Server-only, from BeginPlay)
  (message `/Game/MMOKit/MMO_Logic/Blueprints/Interfaces/BPI_MobSpecific.OnPlayerLeftAggro` OtherActor self))

(event `SetupComponents`
  ;[1 0.312 0.302] SetupComponents: Destroys the components of the current camera type and adds the desired components
  (`MmoUtilities.LogString` "Character: Setup Components")
  (`/Engine/EditorBlueprintResources/StandardMacros.Can Execute Cosmetic Events`
    (:`True`
      (`|ExecutionSequence`
        (:`then_0`
          (`/Game/MMOKit/MMO_Logic/Blueprints/BPFL_Lib.DestroyComponentIfValid` (`self.CameraTypeComponent`))
          (`/Game/MMOKit/MMO_Logic/Blueprints/BPFL_Lib.DestroyComponentIfValid` (`self.InteractionSystemComponent`)))
        (:`then_1`
          (bind _returnvalue (`|AddComponentByClass` (select `/Game/MMOKit/MMO_Logic/Blueprints/Enums/ECameraType` (`/Game/MMOKit/MMO_Logic/Blueprints/BP_PlayerController.CameraType` (`self.GetBpController`)) :`NewEnumerator0` "/Game/MMOKit/MMO_Logic/Blueprints/Camera/BP_FirstPersonCameraComponent.BP_FirstPersonCameraComponent_C" :`NewEnumerator1` "/Game/MMOKit/MMO_Logic/Blueprints/Camera/BP_OverShoulderCameraComponent.BP_OverShoulderCameraComponent_C" :`NewEnumerator2` "/Game/MMOKit/MMO_Logic/Blueprints/Camera/BP_WowStyleCameraComponent.BP_WowStyleCameraComponent_C" :!type "ActorComponent Class Reference")))
          (bind _asbp_base_camera_component (cast `/Game/MMOKit/MMO_Logic/Blueprints/Camera/BP_BaseCameraComponent` _returnvalue))
          (set `self.CameraTypeComponent` _asbp_base_camera_component)
          (bind _returnvalue_2 (`|AddComponentByClass` (select `/Game/MMOKit/MMO_Logic/Blueprints/Enums/ECameraType` (`/Game/MMOKit/MMO_Logic/Blueprints/BP_PlayerController.CameraType` (`self.GetBpController`)) :`NewEnumerator0` "/Game/MMOKit/MMO_Logic/Blueprints/Interaction/BP_InteractionFirstThirdPerson.BP_InteractionFirstThirdPerson_C" :`NewEnumerator1` "/Game/MMOKit/MMO_Logic/Blueprints/Interaction/BP_InteractionFirstThirdPerson.BP_InteractionFirstThirdPerson_C" :`NewEnumerator2` "/Game/MMOKit/MMO_Logic/Blueprints/Interaction/BP_InteractionWowStyle.BP_InteractionWowStyle_C" :!type "ActorComponent Class Reference")))
          (bind _asbp_interaction_system_base (cast `/Game/MMOKit/MMO_Logic/Blueprints/Interaction/BP_InteractionSystemBase` _returnvalue_2))
          (set `self.InteractionSystemComponent` _asbp_interaction_system_base))
        (:`then_2`
          (bind _eventbus (message `/Game/MMOKit/MMO_Logic/Blueprints/Interfaces/BPI_PlayerController.GetPlayerControllerEventBus` (`GameplayStatics.GetPlayerController` 0)))
          (`/Game/MMOKit/MMO_Logic/Blueprints/EventBuses/BP_PlayerControllerEventBus.OnCharacterReadyClient` _eventbus) ; Always notify that we've (re-)set up our components
        )))))

(event `SetActorRotationOnServer`
  (params (NewRot :type "Rotator Structure"))
  ;[0.4452 0.6332 1] Events used by camera components to replicate correct character rotation to others
  (`self.K2_SetActorRotation` NewRot))

(event `SetUseControllerRotationOnServer`
  (params (Use :type Boolean))
  ;[0.4452 0.6332 1] Events used by camera components to replicate correct character rotation to others
  (set `CharacterMovementComponent.bUseControllerDesiredRotation` Use (`self.CharacterMovement`)))

(event `SetRotationRateOnServer`
  (params (RotRate :type "Float (double-precision)"))
  ;[0.4452 0.6332 1] Events used by camera components to replicate correct character rotation to others
  (set `CharacterMovementComponent.RotationRate` (`KismetMathLibrary.MakeRotator` 0.0 0.0 RotRate) (`self.CharacterMovement`)))

(event `/Game/MMOKit/MMO_Logic/Blueprints/Interfaces/BPI_Character.Resurrect`
  ;[0.4452 0.6332 1] Resurrect: extends parent's function to teleport to graveyard
  (`parent.Resurrect`)
  (bind _location (`self.GetNearestGraveyard`))
  (`self.K2_TeleportTo` (+ _location (`KismetMathLibrary.MakeVector` 0.0 0.0 (`CapsuleComponent.CapsuleHalfHeight` (`self.CapsuleComponent`)))) (`KismetMathLibrary.MakeRotator` 0.0 0.0 (`KismetMathLibrary.RandomFloatInRange` 0.0 360.0)))
  (bind _eventbus (message `/Game/MMOKit/MMO_Logic/Blueprints/Interfaces/BPI_PlayerController.GetPlayerControllerEventBus` (`self.GetController`) :!label _label_3))
  (`/Game/MMOKit/MMO_Logic/Blueprints/EventBuses/BP_PlayerControllerEventBus.OnCharacterResurrected` _eventbus))

(event `/Game/MMOKit/MMO_Logic/Blueprints/Interfaces/BPI_FirstPersonCharacter.EmitUpdateHands`
  (params (RHand :type "PrimaryAssetId Structure") (Appearance :type "/Game/MMOKit/MMO_Logic/Blueprints/DataAssetTypes/CreatureAppearance Object Reference") (Sex :type "/Game/MMOKit/MMO_Logic/Blueprints/Enums/ECreatureSex Enum" :default "NewEnumerator0"))
  ;[1 0.312 0.302] Interface implementation for FirstPersonCharacter
  (`/Engine/EditorBlueprintResources/StandardMacros.Can Execute Cosmetic Events`
    (:`True`
      (`self.IsOurCharacter`
        (:`Yes`
          (if (`self.ComponentsAreSetUp`) :!label _label_4
            (`MmoUtilities.LogString` "Appearance: UpdateHands")
            (`self.OnHandsUpdated` RHand Appearance Sex)
            (else
              (`KismetSystemLibrary.DelayUntilNextTick`)
              (`MmoUtilities.LogString` "Appearance: delaying UpdateHands by 1 frame")
              (goto _label_4))))))))

(event `self.Resurrect_Multicast`
  ;[1 0.312 0.302] Resurrect_Multicast: extends parent
  (`parent.Resurrect_Multicast`)
  (`/Engine/EditorBlueprintResources/StandardMacros.Can Execute Cosmetic Events`
    (:`True`
      (`self.IsOurCharacter`
        (:`Yes`
          (goto _label_3))))))

(event `/Game/MMOKit/MMO_Logic/Blueprints/Interfaces/BPI_Character.Die`
  (params (Killer :type "Character Object Reference"))
  ;[0.4452 0.6332 1] Die: extends parent's function
  (`parent.Die` Killer)
  ;[0.7865 0.1065 0.7201] call OnCharacterDied dispatcher
  (bind _eventbus (message `/Game/MMOKit/MMO_Logic/Blueprints/Interfaces/BPI_PlayerController.GetPlayerControllerEventBus` (`self.GetController`) :!label _label_5))
  (`/Game/MMOKit/MMO_Logic/Blueprints/EventBuses/BP_PlayerControllerEventBus.OnCharacterDied` _eventbus))

(event `DestroyComponent`
  (params (CompToDestroy :type "ActorComponent Object Reference"))
  ;[1 1 1] Destroy child component
  ; Called by other components to manage the parent
  (`/Game/MMOKit/MMO_Logic/Blueprints/BPFL_Lib.DestroyComponentIfValid` CompToDestroy))

(event `self.Die_Multicast`
  ;[1 0.312 0.302] Die_Multicast: extends parent's function
  (`parent.Die_Multicast`)
  (`/Engine/EditorBlueprintResources/StandardMacros.Can Execute Cosmetic Events`
    (:`True`
      (`self.IsOurCharacter`
        (:`Yes`
          (goto _label_5))))))

(event `/Game/MMOKit/MMO_Logic/Blueprints/Interfaces/BPI_PlayerCharacterSpecific.ChangeReactionToCreature`
  (params (Aggro :type Boolean) (Char :type "Character Object Reference"))
  ;[0.4452 0.6332 1] ChangeReactionToCreature: mobs that
  ; have added us to their aggro will send
  ; us this notification from server
  (`self.ChangeReactionToCreatureClient` Aggro Char))

(event `ChangeReactionToCreatureClient`
  (params (Aggro :type Boolean) (Char :type "Character Object Reference"))
  ;[1 0.312 0.302] ChangeReactionToCreatureClient
  (if Aggro
    (message `/Game/MMOKit/MMO_Logic/Blueprints/Interfaces/BPI_Reaction.SetLocalReaction` Char "NewEnumerator2")
    (else
      (bind _isplayer (message `/Game/MMOKit/MMO_Logic/Blueprints/Interfaces/BPI_Character.IsPlayerCharacter` Char))
      (if _isplayer
        (message `/Game/MMOKit/MMO_Logic/Blueprints/Interfaces/BPI_Reaction.SetLocalReaction` Char "NewEnumerator0")
        (else
          (bind _reaction (message `/Game/MMOKit/MMO_Logic/Blueprints/Interfaces/BPI_MobSpecific.GetMobInitialReaction` Char))
          (message `/Game/MMOKit/MMO_Logic/Blueprints/Interfaces/BPI_Reaction.SetLocalReaction` Char _reaction))))))

(fn `GetBpController`
  (returns (BpController :type "/Game/MMOKit/MMO_Logic/Blueprints/BP_PlayerController Object Reference"))
  (bind _asbp_player_controller (cast `/Game/MMOKit/MMO_Logic/Blueprints/BP_PlayerController` (`self.GetController`))
    (:`then`
      (return _asbp_player_controller))
    (:`CastFailed`
      (`MmoUtilities.LogString` "GetBpController: null" "Verbosity_Normal" true true (struct :`R` 1.0 :`B` 0.02448 :`A` 1.0) 5.0)
      (return null))))

(fn `GetCharacterEventBus`
  (returns (CharacterEventBus :type "/Game/MMOKit/MMO_Logic/Blueprints/EventBuses/BP_CharacterEventBus Object Reference"))
  (return (`self.EventBus`)))

(fn `GetMeleeAttackOrigin`
  (returns (Origin :type "Transform Structure"))
  (bind _origin (`/Game/MMOKit/MMO_Logic/Blueprints/Camera/BP_BaseCameraComponent.Get Camera Attack Origin` (`self.CameraTypeComponent`)))
  (return _origin))

(fn `GetNearestGraveyard`
  (returns (Location :type "Vector Structure"))
  (locals (NearestGraveyard :type "Actor Object Reference"))
  ;[0.4452 0.6332 1] Get nearest graveyard (they exist only on server)
  (bind _outactors (`GameplayStatics.GetAllActorsOfClass` "/Game/MMOKit/MMO_Logic/Blueprints/Misc/BP_Graveyard.BP_Graveyard_C"))
  (bind _output_get (set `local.NearestGraveyard` (`.ReturnValue` (`GameplayStatics.FindNearestActor` (`self.K2_GetActorLocation`) _outactors))))
  (`/Engine/EditorBlueprintResources/StandardMacros.IsValid` _output_get
    (:`Is Valid`
      (return (`self.K2_GetActorLocation` _output_get)))
    (:`Is Not Valid`
      (return (0.0 0.0 0.0)))))

(fn `GetPlayerCharEventBus`
  (returns (EventBus :type "/Game/MMOKit/MMO_Logic/Blueprints/EventBuses/BP_PlayerCharEventBus Object Reference"))
  (return (`self.EventBus`)))

(fn `GetPlayerStats`
  (returns (PlayerStats :type "/Game/MMOKit/MMO_Logic/Blueprints/Stats/BP_PlayerStatsComponent Object Reference"))
  (return (`self.StatsComp`)))

(fn `GetReaction`
  (returns (Reaction :type "/Game/MMOKit/MMO_Logic/Blueprints/Enums/EReaction Enum"))
  (return "NewEnumerator0"))

(fn `GetStatsComponent`
  (returns (StatsComp :type "/Game/MMOKit/MMO_Logic/Blueprints/Stats/BP_BaseStatsComponent Object Reference"))
  (return (`self.StatsComp`)))

(fn `GetTarget`
  (returns (TargetCharacter :type "Character Object Reference"))
  (bind _asbp_interaction_wow_style (cast `/Game/MMOKit/MMO_Logic/Blueprints/Interaction/BP_InteractionWowStyle` (`self.InteractionSystemComponent`))
    (:`then`
      (return (`/Game/MMOKit/MMO_Logic/Blueprints/Interaction/BP_InteractionWowStyle.SelectedCharacter` _asbp_interaction_wow_style)))
    (:`CastFailed`
      (return null))))

(fn `IsPlayerCharacter`
  (returns (IsPlayer :type Boolean))
  (return true))

(fn `RaycastMeleeAttack`
  (params (FromWhere :type "Transform Structure") (Reach :type "Float (double-precision)") (RaycastWidth :type "Float (double-precision)"))
  (returns (StatsComponent :type "/Game/MMOKit/MMO_Logic/Blueprints/Stats/BP_BaseStatsComponent Object Reference"))
  (bind _statscomponent (`parent.RaycastMeleeAttack` FromWhere Reach RaycastWidth))
  (return _statscomponent))

(fn `SetBody`
  (params (NewMesh :type "SkeletalMesh Object Reference") (AnimBp :type "AnimInstance Class Reference") (Sex :type "/Game/MMOKit/MMO_Logic/Blueprints/Enums/ECreatureSex Enum" :default "NewEnumerator0") (CreRace :type "/Game/MMOKit/MMO_Logic/Blueprints/Enums/ECreatureRace Enum" :default "NewEnumerator2"))
  (returns (Changed :type Boolean))
  (bind _changed (`parent.SetBody` NewMesh AnimBp Sex CreRace))
  (return _changed))

(fn `ShouldAttachEyes`
  (returns (Should :type Boolean))
  (bind _should (`parent.ShouldAttachEyes`))
  (return _should))

(fn `UserConstructionScript`
  (`MmoUtilities.LogString` "Char: construction script")
  (bind _returnvalue (`AddComponent|NODE_AddBP_PlayerCharEventBus-0`))
  (set `self.EventBus` _returnvalue)
  (`/Engine/EditorBlueprintResources/StandardMacros.Can Execute Cosmetic Events`
    (:`False`
      (`/Game/MMOKit/MMO_Logic/Blueprints/BP_AppearanceComponent.InitializePlayerAppearance` (`self.AppearanceComponent`) (`self.InAppearance`))
      (bind _returnvalue_2 (`AddComponent|NODE_AddBP_PlayerStatsComponent-0`))
      (bind _output_get (set `self.StatsComp` _returnvalue_2))
      (`/Game/MMOKit/MMO_Logic/Blueprints/Stats/BP_PlayerStatsComponent.Initialize` _output_get (`self.InStats`))
      (bind _returnvalue_3 (`AddComponent|NODE_AddSphereComponent-2`))
      (bind _output_get_2 (set `self.AggroRangeSphereCollider` _returnvalue_3))
      (`SphereComponent.SetSphereRadius` _output_get_2 500.0 false)
      (`PrimitiveComponent.SetCollisionProfileName` _output_get_2 "AggroSphere" true)
      (add `PrimitiveComponent.OnComponentBeginOverlap` _output_get_2 (`|CreateDelegate` :!event `OnAggroSphereBeginOverlap`))
      (add `PrimitiveComponent.OnComponentEndOverlap` _output_get_2 (`|CreateDelegate` :!event `OnAggroSphereEndOverlap`)))))