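; Player state Blueprint for the MMO kit that preloads ability assets on game instances that run cosmetic events.
; On BeginPlay, it checks CanExecuteCosmeticEvents, then fetches a primary asset ID list and loads it asynchronously through the Asset Manager.
; When loading completes, each result that casts to AbilityAsset is stored in LoadedAbilities and logged at super-verbose level.
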(event `self.ReceiveBeginPlay`
  ;[1 0.312 0.302] Loads AbilityAssets
  (`MmoUtilities.LogString` "BeginPlay: PlayerState")
  (`/Engine/EditorBlueprintResources/StandardMacros.Can Execute Cosmetic Events`
    (:`True`
      (bind _outprimaryassetidlist (`KismetSystemLibrary.GetPrimaryAssetIdList` "AbilityAsset"))
      (bind _loaded (`AsyncActionLoadPrimaryAssetList.AsyncLoadPrimaryAssetList` _outprimaryassetidlist)
        (:`Completed`
          (for _array_element _loaded
            (bind _asability_asset (cast `/Game/MMOKit/MMO_Logic/Blueprints/DataAssetTypes/AbilityAsset` _array_element))
            (`KismetArrayLibrary.Array_Add` (`self.LoadedAbilities`) _asability_asset)
            (`MmoUtilities.LogString` (`KismetStringLibrary.Concat_StrStr` "Client Loaded Ability: " (`KismetSystemLibrary.GetObjectName` _asability_asset)))))))))

(fn `UserConstructionScript`)