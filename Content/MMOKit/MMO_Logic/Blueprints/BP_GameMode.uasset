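; Server game mode for the MMO kit that brokers character loading and saving between player controllers and the persistence server.
; Character requests go out over the game state's TCP connection, with replies matched to controllers through a first-in, first-out queue.
; It preloads item, ability and appearance assets, spawns delayed mob spawners and tracks online characters by name.
; In editor, it warns about setup problems and saves characters when PIE ends.
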(event `/Game/MMOKit/MMO_Logic/Blueprints/Interfaces/BPI_GameMode.GetCharacterForController`
  (params (PlayerController :type "PlayerController Object Reference") (Cookie :type String) (CharID :type Integer))
  ;[0.4452 0.6332 1] This all has to do with when we GetCharacter from Persistence server
  (`KismetArrayLibrary.Array_Add` (`self.GetCharacterQueue`) PlayerController)
  (bind _tcpconn (message `/Game/MMOKit/MMO_Logic/Blueprints/Interfaces/BPI_GameState.GetTcpConnection` (`GameplayStatics.GetGameState`)))
  (`/Game/MMOKit/MMO_Logic/Blueprints/TCP/BP_TcpConnection.GetCharacter` _tcpconn Cookie CharID)
  ;[1 1 1] Editor only: display warning if user hasn't launched the persistence server
  (bind _returnvalue (`MmoUtilities.InPieWorld`))
  (if _returnvalue
    (if (not (`TcpSocketConnection.isConnected` _tcpconn 0))
      (message `/Game/MMOKit/MMO_Logic/Blueprints/Interfaces/BPI_PlayerController.DisplayEditorWarning1` PlayerController))))

(event `/Game/MMOKit/MMO_Logic/Blueprints/Interfaces/BPI_GameMode.FailedGettingCharacterForController`
  (bind _getcharacterqueue (`self.GetCharacterQueue`))
  (bind _getcharacterqueue_2 (`self.GetCharacterQueue`))
  ;[0.4452 0.6332 1] This all has to do with when we GetCharacter from Persistence server
  (bind _returnvalue (`MmoUtilities.InPieWorld`))
  (if _returnvalue
    ;;[1 1 1] in editor, display a warning that there's not enough characters in DB
    (message `/Game/MMOKit/MMO_Logic/Blueprints/Interfaces/BPI_PlayerController.DisplayEditorWarning2` (`|GetArrayItem` _getcharacterqueue))
    (`KismetArrayLibrary.Array_Remove` _getcharacterqueue)
    (else
      ;;[0.4452 0.6332 1] in prod, disconnect player
      (`self.K2_DestroyActor` (`|GetArrayItem` _getcharacterqueue_2))
      (`KismetArrayLibrary.Array_Remove` _getcharacterqueue_2))))

(event `/Game/MMOKit/MMO_Logic/Blueprints/Interfaces/BPI_GameMode.SpawnMobAfterDelay`
  (params (RespawnPoint :type "Transform Structure") (MobClass :type "/Game/MMOKit/MMO_Logic/Blueprints/BP_MobCharacter Class Reference") (Stats :type "/Game/MMOKit/MMO_Logic/Blueprints/Struct/FStatsMob Structure") (Delay :type "Float (double-precision)") (Loot :type "/Game/MMOKit/MMO_Logic/Blueprints/Struct/FMobLoot Structure") (BT :type "BehaviorTree Object Reference"))
  ;[0.4452 0.6332 1] Spawn mob after a delay
  (`|SpawnActorFromClass` "/Game/MMOKit/MMO_Logic/Blueprints/Misc/BP_MobSpawner.BP_MobSpawner_C" RespawnPoint "AlwaysSpawn" "OverrideRootScale" null MobClass Stats Delay Loot BT null))

(event `/Game/MMOKit/MMO_Logic/Blueprints/Interfaces/BPI_GameMode.GotCharacterForController`
  (params (AccountID :type Integer) (CharID :type Integer) (CharName :type String) (Serialized :type String) (GuildId :type Integer) (GuildRank :type Integer))
  (bind _getcharacterqueue (`self.GetCharacterQueue`))
  ;[0.4452 0.6332 1] This all has to do with when we GetCharacter from Persistence server
  (bind _eventbus (message `/Game/MMOKit/MMO_Logic/Blueprints/Interfaces/BPI_PlayerController.GetPlayerControllerEventBus` (`|GetArrayItem` _getcharacterqueue)))
  (`/Game/MMOKit/MMO_Logic/Blueprints/EventBuses/BP_PlayerControllerEventBus.OnGotCharacterFromDB` _eventbus AccountID CharID CharName Serialized GuildId GuildRank)
  (`KismetArrayLibrary.Array_Remove` _getcharacterqueue))

(event `/Game/MMOKit/MMO_Logic/Blueprints/Interfaces/BPI_GameMode.ContinuePlayerSpawn`
  (params (PlayerController :type "/Game/MMOKit/MMO_Logic/Blueprints/BP_PlayerController Object Reference") (PlayerPawn :type "Pawn Object Reference") (SpawnRotator :type "Rotator Structure"))
  ;[0.4452 0.6332 1] This all has to do with when we GetCharacter from Persistence server
  (`self.ContinuePlayerStart` PlayerController PlayerPawn SpawnRotator))

(event `self.ReceiveBeginPlay`
  ;[0.4452 0.6332 1] Server-side: Load assets and keep them in memory by referencing them in the game mode
  (`|ExecutionSequence`
    (:`then_0`
      (`MmoUtilities.LogString` "BeginPlay: GameMode")
      (for _array_element (`self.PrimaryTypesToLoad`)
        (bind _outprimaryassetidlist (`KismetSystemLibrary.GetPrimaryAssetIdList` _array_element))
        (bind _loaded (`AsyncActionLoadPrimaryAssetList.AsyncLoadPrimaryAssetList` _outprimaryassetidlist)
          (:`Completed`
            (for _array_element_2 _loaded
              (bind _asitem_asset (cast `ItemAsset` _array_element_2)
                (:`then`
                  (`KismetArrayLibrary.Array_Add` (`self.LoadedItems`) _asitem_asset)
                  (`MmoUtilities.LogString` (`KismetStringLibrary.Concat_StrStr` "Server Loaded Item: " (`KismetTextLibrary.Conv_TextToString` (`ItemAsset.ItemName` _asitem_asset)))))
                (:`CastFailed`
                  (bind _asability_asset (cast `/Game/MMOKit/MMO_Logic/Blueprints/DataAssetTypes/AbilityAsset` _array_element_2)
                    (:`then`
                      (`KismetArrayLibrary.Array_Add` (`self.LoadedAbilities`) _asability_asset)
                      (`MmoUtilities.LogString` (`KismetStringLibrary.Concat_StrStr` "Server Loaded Ability: " (`KismetSystemLibrary.GetObjectName` _asability_asset))))
                    (:`CastFailed`
                      (bind _ascreature_appearance (cast `/Game/MMOKit/MMO_Logic/Blueprints/DataAssetTypes/CreatureAppearance` _array_element_2))
                      (`KismetArrayLibrary.Array_Add` (`self.LoadedAppearances`) _ascreature_appearance)
                      (`MmoUtilities.LogString` (`KismetStringLibrary.Concat_StrStr` "Server Loaded Appearance: " (`KismetSystemLibrary.GetObjectName` _ascreature_appearance))))))))))))
    (:`then_1`
      ;;[1 1 1] If launching the project in an incorrect mode, display a warning for user
      (if (and (`KismetSystemLibrary.IsServer`) (not (`KismetSystemLibrary.IsDedicatedServer`)))
        (`KismetSystemLibrary.Delay` 1.0)
        (message `/Game/MMOKit/MMO_Logic/Blueprints/Interfaces/BPI_PlayerController.DisplayEditorWarning3` (`GameplayStatics.GetPlayerController` 0))))))

(event `self.K2_OnEndPIE`
  ;[0.4452 0.6332 1] OnEndPIE gets fired only in Editor
  ; In a regular game, PlayerController::OnUnPossess will save the exiting character
  ; But in Editor, UnPossess will fire so late,  that our TCP connection will already be closed
  ; So we fire attempt to save characters as soon as PIE ends
  (`self.SaveAllCharacters`))

(event `SaveAllCharacters`
  ;[0.4452 0.6332 1] Save All Characters
  (`MmoUtilities.LogString` "Saving All Characters")
  (for _index (range (`GameplayStatics.GetNumPlayerControllers`))
    (message `/Game/MMOKit/MMO_Logic/Blueprints/Interfaces/BPI_PlayerController.ForceSaveCharacter` (`GameplayStatics.GetPlayerController` _index))))

(event `/Game/MMOKit/MMO_Logic/Blueprints/Interfaces/BPI_GameMode.SaveCharacter`
  (params (ChId :type Integer) (Json :type "JsonObjectWrapper Structure"))
  ;[0.4452 0.6332 1] Save Character - gets called from PlayerController
  (bind _tcpconn (message `/Game/MMOKit/MMO_Logic/Blueprints/Interfaces/BPI_GameState.GetTcpConnection` (`GameplayStatics.GetGameState`)))
  (`/Game/MMOKit/MMO_Logic/Blueprints/TCP/BP_TcpConnection.SaveCharacter` _tcpconn ChId Json))

(event `/Game/MMOKit/MMO_Logic/Blueprints/Interfaces/BPI_GameMode.CharacterEnteredWorld`
  (params (Name :type String) (Character :type "Character Object Reference"))
  (`BlueprintMapLibrary.Map_Add` (`self.CharactersOnline`) Name Character))

(event `/Game/MMOKit/MMO_Logic/Blueprints/Interfaces/BPI_GameMode.CharacterLeftWorld`
  (params (Name :type String))
  (`BlueprintMapLibrary.Map_Remove` (`self.CharactersOnline`) Name))

(fn `GetPlayerCharByName`
  (params (Charname :type String))
  (returns (PlayerChar :type "Character Object Reference") (Found :type Boolean))
  (bind (_value _returnvalue) (`BlueprintMapLibrary.Map_Find` (`self.CharactersOnline`) Charname))
  (return _value _returnvalue))

(fn `GetServerPassword`
  (returns (Password :type String))
  (return (`self.ServerPassword`)))

(fn `UserConstructionScript`)